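; Gridworld level prop that displays a configurable glowing static mesh, styled as either hex tech or neon edge.
; The construction script assigns the chosen mesh, then selects a material by the hex and static-light flags.
; Static lights push the chosen light color into the material's emissive color parameter, while non-static lights use pulse material variants without setting a color.
; There is no runtime logic.
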(event EventBeginPlay)

(fn ConstructionScript
  (bind _staticmesh (Variables|Default|GetStaticMesh))
  (bind _staticmesh_2 (Variables|Default|GetStaticMesh))
  (Components|StaticMesh|SetStaticMesh (Variables|Default|GetStaticMesh) (Variables|Default|GetMeshToUse))
  (if (Variables|Default|GetUseHex)
    (if (Variables|Default|GetStaticLights)
      (Rendering|Material|SetMaterial _staticmesh_2 0 "/Game/Materials/HexTech_M.HexTech_M")
      (Rendering|Material|SetVectorParameterValueonMaterials _staticmesh_2 "Emissive color" (Math|Conversions|ToVector(LinearColor) (Variables|Default|GetLightColor)))
      (else
        (Rendering|Material|SetMaterial _staticmesh_2 0 "/Game/Materials/HexTech_Pulse_M.HexTech_Pulse_M")))
    (elif (Variables|Default|GetStaticLights)
      (Rendering|Material|SetMaterial _staticmesh 0 "/Game/Materials/NeonEdge_M.NeonEdge_M")
      (Rendering|Material|SetVectorParameterValueonMaterials _staticmesh "Emissive color" (Math|Conversions|ToVector(LinearColor) (Variables|Default|GetLightColor)))
      (else
        (Rendering|Material|SetMaterial _staticmesh 0 "/Game/Materials/NeonEdge_Pulse_M.NeonEdge_Pulse_M")))))