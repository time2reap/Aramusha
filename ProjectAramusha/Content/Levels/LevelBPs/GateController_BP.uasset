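; Gate controller Blueprint that toggles a kill wall, with two blinkers flashing as a warning.
; Starting on or turning on runs a timed blink sequence before enabling the KillWall, while turning off disables it and fades the blinkers out.
; A timeline played forward and in reverse drives blinker opacity and glow.
; The random-open option only waits and re-rolls its delay, without calling the turn-off event.
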(event Custom|Turn%20Gate%20Off
  (Default|TurnOff (Variables|Default|GetKillWall))
  (CallFunction|BlinkerFadeOff))

(event Custom|Turn%20Gate%20On
  (CallFunction|BlinkerFadeOff)
  (Utilities|FlowControl|Delay 1.0)
  (CallFunction|BlinkerFadeon)
  (Utilities|FlowControl|Delay 1.0)
  (CallFunction|BlinkerFadeOff)
  (Utilities|FlowControl|Delay 1.0)
  (CallFunction|BlinkerFadeon)
  (Utilities|FlowControl|Delay 1.0)
  (Default|Turnon (Variables|Default|GetKillWall))
  (if (Variables|Default|GetRandomlyOpen)
    (Utilities|FlowControl|Delay (Variables|Default|GetOpenDelay))
    (Variables|Default|SetOpenDelay (Math|Random|RandomFloatinRange (Variables|Default|GetMinDelay) (Variables|Default|GetMaxDelay)))))

(event Custom|BlinkerFadeOn
  (bind _blinker1 (Variables|Default|GetBlinker1))
  (bind _delta (Timeline|FadeTL PlayFromStart)
    (:Update
      (Rendering|Material|SetScalarParameterValueonMaterials _blinker1 "Opacity" _delta)
      (Rendering|Material|SetScalarParameterValueonMaterials _blinker1 "Glow Strength" (* _delta (Variables|Default|GetGlowStrength))))))

(event Custom|BlinkerFadeOff
  (bind _blinker1 (Variables|Default|GetBlinker1))
  (bind _delta (Timeline|FadeTL ReverseFromEnd)
    (:Update
      (Rendering|Material|SetScalarParameterValueonMaterials _blinker1 "Opacity" _delta)
      (Rendering|Material|SetScalarParameterValueonMaterials _blinker1 "Glow Strength" (* _delta (Variables|Default|GetGlowStrength))))))

(event EventBeginPlay
  (if (Variables|Default|GetStartOn)
    (Default|TurnOff (Variables|Default|GetKillWall))
    (CallFunction|TurnGateon)
    (else
      (CallFunction|TurnGateOff)))
  (if (Variables|Default|GetRandomlyOpen)
    (Variables|Default|SetOpenDelay (Math|Random|RandomFloatinRange (Variables|Default|GetMinDelay) (Variables|Default|GetMaxDelay)))))

(fn ConstructionScript)