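; Paired teleporter actor that moves a player character entering its collider to the location and rotation of its partner.
; On BeginPlay it links to the first other Teleporter_BP sharing its Channel.
; Linking and overlap handling run only on the Remote (non-authority) branch, calling the character's RPCTeleport and deactivating both ends for TPDelay to prevent bouncing back.
; The construction script tints the glow cylinder, arrow and point light with Color.
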(event OnComponentBeginOverlap(Collider)
  (params (OverlappedComponent :type Primitive%20Component%20Object%20Reference) (OtherActor :type Actor%20Object%20Reference) (OtherComp :type Primitive%20Component%20Object%20Reference) (OtherBodyIndex :type Integer) (bFromSweep :type Boolean) (SweepResult :type Hit%20Result%20Structure%20%28by%20ref%29))
  (bind _othertp (Variables|Default|GetOtherTP))
  (Networking|SwitchHasAuthority
    (:Remote
      (if (Variables|Default|GetActive)
        (bind _asplayer_character (Utilities|Casting|CastToPlayerCharacter OtherActor))
        (Variables|Default|SetActive false)
        (Variables|Teleporter_BP_C|SetActive _othertp false)
        (Default|RPCTeleport _asplayer_character (Transformation|GetActorLocation _othertp) (Transformation|GetActorRotation _othertp))
        (Utilities|FlowControl|Delay (Variables|Default|GetTP_Delay))
        (Variables|Default|SetActive true)
        (Variables|Teleporter_BP_C|SetActive _othertp true)))))

(event Custom|Init
  (bind _outactors (Actor|GetAllActorsOfClass "Teleporter_BP_C"))
  (bind _array_element (Utilities|Array|ForEachLoopwithBreak _outactors :!label _label)
    (:LoopBody
      (if (and (Utilities|Enum|Equal(Enum) (Variables|Teleporter_BP_C|GetChannel _array_element) (Variables|Default|GetChannel)) (!= _array_element self))
        (Variables|Default|SetOtherTP _array_element)
        (goto _label Break)))))

(event EventBeginPlay
  (Networking|SwitchHasAuthority
    (:Remote
      (CallFunction|Init))))

(fn ConstructionScript
  (bind _color (Variables|Default|GetColor))
  (Rendering|Material|SetVectorParameterValueonMaterials (Variables|Default|GetglowCylinder) "EmissiveColor" (Math|Conversions|ToVector(LinearColor) _color))
  (Rendering|Components|Light|SetLightColor (Variables|Default|GetPointLight) _color true))