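; Floating object actor for levels that continuously spins and bobs along a looping path.
; Each Tick, RotateAndMove advances a timer that wraps at FloatCycleTime and adds RotationSpeed to the rotation per frame, unscaled by delta time.
; GetCosineInterp turns cycle progress into a raw -1 to 1 cosine, which scales the MaxHeight–MinHeight difference around MinHeight to set the absolute location.
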(event EventBeginPlay)

(event Collision|EventActorBeginOverlap
  (params (OtherActor :type Actor%20Object%20Reference)))

(event EventTick
  (params (DeltaSeconds :type Float%20%28single-precision%29))
  (CallFunction|RotateandMove DeltaSeconds))

(fn ConstructionScript)

(fn RotateandMove
  (params (deltaTime :type Float%20%28single-precision%29))
  (Variables|Default|SetcurrentTime (+ (Variables|Default|GetcurrentTime) deltaTime))
  ;[1 1 1] Resetting the timer when it goes past the max cycle time
  (if (not (>= (Variables|Default|GetcurrentTime) (Variables|Default|GetfloatCycleTime)))
    _
    (else
      (Variables|Default|SetcurrentTime (- (Variables|Default|GetcurrentTime) (Variables|Default|GetfloatCycleTime)))))
  ;[1 1 1] Rotating this actor each tick
  (Transformation|SetActorRotation (Math|Rotator|CombineRotators (Variables|Default|GetrotationSpeed) (Transformation|GetActorRotation)))
  (bind _cospercent (CallFunction|GetCosineInterp))
  (bind _output_get (LocalVariables|SetposDiff (* (- (Variables|Default|GetmaxHeight) (Variables|Default|GetminHeight)) _cospercent)))
  (bind _output_get_2 (LocalVariables|SetposDiff (+ (Variables|Default|GetminHeight) _output_get)))
  (Transformation|SetActorLocation _output_get_2 false false))

(fn GetCosineInterp
  (bind _output_get (LocalVariables|SettimePercent (* (/ (Variables|Default|GetcurrentTime) (Variables|Default|GetfloatCycleTime)) 3.6e+02)))
  (return (Math|Trig|Cos(Degrees) _output_get)))