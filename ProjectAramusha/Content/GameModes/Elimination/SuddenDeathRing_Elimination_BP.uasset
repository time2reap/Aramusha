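; Shrinking sudden-death safe zone for Elimination mode that kills players who leave it.
; On BeginPlay the authority caches the game mode, moves the ring to a random CenterLocations entry (or the origin) and hides it at zero scale.
; ActivateSuddenDeath restores the starting size, then Tick scales the actor down linearly with remaining time.
; While active, players ending overlap with SphereSafeZone are passed to the game mode's KillPlayer.
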(event OnComponentEndOverlap(SphereSafeZone)
  (params (OverlappedComponent :type Primitive%20Component%20Object%20Reference) (OtherActor :type Actor%20Object%20Reference) (OtherComp :type Primitive%20Component%20Object%20Reference) (OtherBodyIndex :type Integer))
  ;[1 0.1497 0.9863] End Overlap
  (if (Variables|Default|GetisActive)
    ;;[1 1 1] Telling our game mode to kill the player that left the safe zone during sudden death
    (bind _asplayer_character (Utilities|Casting|CastToPlayerCharacter OtherActor))
    (Default|KillPlayer (Variables|Default|GetgameMode) _asplayer_character)))

(event Custom|ActivateSuddenDeath
  ;[1 0.8726 0.09549] Activate Sudden Death
  ;;[1 1 1] Setting the starting size and timer for sudden death
  (Variables|Default|SetisActive true)
  (Transformation|SetActorScale3D (Variables|Default|GetstartingSize))
  (Variables|Default|SetcurrentSuddenDeathTime (Variables|Default|GetsuddenDeathDuration)))

(event EventBeginPlay
  (bind _centerlocations (Variables|Default|GetcenterLocations))
  ;[0.1175 1 0.1248] Begin Play
  (Networking|SwitchHasAuthority
    (:Authority
      (bind _aselimination_game_mode (Utilities|Casting|CastToElimination_GameMode (Variables|/Script/Engine.GameStateBase|GetAuthorityGameMode (Game|GetGameState))))
      (Variables|Default|SetgameMode _aselimination_game_mode)
      (if (> (Utilities|Array|Length (Variables|Default|GetcenterLocations)) 0)
        ;;[1 1 1] Setting the center location to a random index in the array
        (Transformation|SetActorLocation (Utilities|Array|Get(acopy) _centerlocations (Math|Random|RandomInteger (- (Utilities|Array|Length _centerlocations) 1))) false true)
        (else
          ;;[1 1 1] If there are no valid center locations, we set the center to 0,0,0
          (Transformation|SetActorLocation "0, 0, 0" false true)))
      (Transformation|SetActorScale3D "0, 0, 0"))))

(event EventTick
  (params (DeltaSeconds :type Float%20%28single-precision%29))
  ;[0.1043 0.8702 1] Tick
  (if (Variables|Default|GetisActive)
    ;;[1 1 1] Counting down the sudden death timer and shrinking our death ring
    (bind _output_get (Variables|Default|SetcurrentSuddenDeathTime (- (Variables|Default|GetcurrentSuddenDeathTime) DeltaSeconds)))
    (Transformation|SetActorScale3D (* (Variables|Default|GetstartingSize) (/ _output_get (Variables|Default|GetsuddenDeathDuration))))))

(fn ConstructionScript)