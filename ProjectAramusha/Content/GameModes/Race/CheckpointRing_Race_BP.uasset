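; Numbered checkpoint ring for the Race game mode that tracks players' progress through the course in order.
; On the server, its cylinder overlap reports living players to Race_GameMode only if their last checkpoint is the preceding one, flagging the finish line.
; On clients, a separate non-replicated cylinder handles visibility: rings after the first start hidden, and the local player's overlap hides the ring and reveals NextCheckpoint unless it is the finish.
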(event OnComponentBeginOverlap(CylinderCollider)
  (params (OverlappedComponent :type Primitive%20Component%20Object%20Reference) (OtherActor :type Actor%20Object%20Reference) (OtherComp :type Primitive%20Component%20Object%20Reference) (OtherBodyIndex :type Integer) (bFromSweep :type Boolean) (SweepResult :type Hit%20Result%20Structure%20%28by%20ref%29))
  ;[0.1244 0.5277 1] Begin Overlap RepCylinder
  (bind _asplayer_character (Utilities|Casting|CastToPlayerCharacter OtherActor))
  (if (not (Variables|/Game/PlayerCharacter/Blueprints/PlayerCharacter.PlayerCharacter_C|GetisDead _asplayer_character))
    (Networking|SwitchHasAuthority
      (:Authority
        ;;[1 1 1] Finding the checkpoint index the player is on
        (bind _playercheckpointnum (Default|GetPlayerCheckpointNum (Variables|Default|GetraceGameModeRef) _asplayer_character))
        (if (!= _playercheckpointnum -1)
          ;;[1 1 1] If the player's current checkpoint is the one before this one, we tell the Race game mode that they made it to the checkpoint
          (if (== (- (Variables|Default|GetcheckpointNum) 1) _playercheckpointnum)
            (Default|PlayerReachedCheckpoint (Variables|Default|GetraceGameModeRef) _asplayer_character (Variables|Default|GetcheckpointNum) (Variables|Default|GetisFinishLine))))))))

(event OnComponentBeginOverlap(NonReplicatedCylinderCollider)
  (params (OverlappedComponent :type Primitive%20Component%20Object%20Reference) (OtherActor :type Actor%20Object%20Reference) (OtherComp :type Primitive%20Component%20Object%20Reference) (OtherBodyIndex :type Integer) (bFromSweep :type Boolean) (SweepResult :type Hit%20Result%20Structure%20%28by%20ref%29))
  ;[1 0.05729 0.05729] Begin Overlap Non-RepCylinder
  (bind _asplayer_character (Utilities|Casting|CastToPlayerCharacter OtherActor))
  (if (not (Variables|/Game/PlayerCharacter/Blueprints/PlayerCharacter.PlayerCharacter_C|GetisDead _asplayer_character))
    (Networking|SwitchHasAuthority
      (:Remote
        (Utilities|IsValid (Variables|/Game/PlayerCharacter/Blueprints/PlayerCharacter.PlayerCharacter_C|GetMyPlayerController _asplayer_character)
          (:Is%20Valid
            (if (Pawn|IsLocalPlayerController (Variables|/Game/PlayerCharacter/Blueprints/PlayerCharacter.PlayerCharacter_C|GetMyPlayerController _asplayer_character))
              ;;[1 1 1] Disabling this ring and enabling the next ring (if this isn't the finish line)
              (CallFunction|SetClientEnable false)
              (if (not (Variables|Default|GetisFinishLine))
                (CallFunction|SetClientEnable (Variables|Default|GetnextCheckpoint) true)))))))))

(event Custom|SetClientEnable
  (params (isEnabled :type Boolean))
  ;[1 0.7944 0.2338] Set Client Enable
  (if isEnabled
    (Components|Activation|SetActive (Variables|Default|GetNonReplicatedCylinderCollider) true false)
    (Development|SetHiddeninGame (Variables|Default|GetNonReplicatedCylinderCollider) false true)
    (else
      (Components|Activation|SetActive (Variables|Default|GetNonReplicatedCylinderCollider) true false)
      (Development|SetHiddeninGame (Variables|Default|GetNonReplicatedCylinderCollider) true true))))

(event EventBeginPlay
  ;[0.1737 1 0.2245] Begin Play
  (Networking|SwitchHasAuthority
    (:Authority
      ;;[1 1 1] If this ring is on the server, we find get a reference to the Race game mode
      (bind _asrace_game_mode (Utilities|Casting|CastToRace_GameMode (Variables|/Script/Engine.GameStateBase|GetAuthorityGameMode (Game|GetGameState)))
        (:then
          (Variables|Default|SetraceGameModeRef _asrace_game_mode))
        (:CastFailed
          (Actor|DestroyActor self))))
    (:Remote
      ;;[1 1 1] If this ring isn't the first ring, we hide it
      (if (> (Variables|Default|GetcheckpointNum) 1)
        (CallFunction|SetClientEnable false)))))

(fn ConstructionScript)