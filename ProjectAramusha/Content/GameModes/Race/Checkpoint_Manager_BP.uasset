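; Checkpoint manager actor for the Race game mode that relays player checkpoint progress to the game mode.
; On BeginPlay the server caches the Race game mode, printing an error if the cast fails.
; UpdatePlayerProgress runs only with authority and reports the player and checkpoint number, flagging a finish at the last CheckpointTransforms index.
; EndRace is an empty stub with its winner message left disconnected.
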(event Custom|UpdatePlayerProgress
  (params (playerToUpdate :type Player%20Character%20Object%20Reference) (checkpointNumber :type Integer))
  (Networking|SwitchHasAuthority
    (:Authority
      (Development|PrintString "CHECKPOINT MANAGER: Update player progress" true true "(R=1.000000,G=0.428228,B=0.000000,A=1.000000)" 1e+01)
      (Default|PlayerReachedCheckpoint (Variables|Default|GetcurrentRaceGameMode) playerToUpdate checkpointNumber (>= checkpointNumber (- (Utilities|Array|Length (Variables|Default|GetcheckpointTransforms)) 1))))))

(event EventBeginPlay
  (Networking|SwitchHasAuthority
    (:Authority
      (bind _asrace_game_mode (Utilities|Casting|CastToRace_GameMode (Variables|/Script/Engine.GameStateBase|GetAuthorityGameMode (Game|GetGameState)))
        (:then
          (Variables|Default|SetcurrentRaceGameMode _asrace_game_mode))
        (:CastFailed
          (Development|PrintString "CAST TO RACE GAME MODE FAILED" true true "(R=1.000000,G=0.000000,B=0.045438,A=1.000000)" 2e+01))))))

(event Collision|EventActorBeginOverlap
  (params (OtherActor :type Actor%20Object%20Reference)))

(event EventTick
  (params (DeltaSeconds :type Float%20%28single-precision%29)))

(fn ConstructionScript)

(fn EndRace
  (params (winningPlayer :type Player%20Character%20Object%20Reference)))