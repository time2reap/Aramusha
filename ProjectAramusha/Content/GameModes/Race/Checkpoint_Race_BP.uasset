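; Race checkpoint ring that relocates itself along the course as the locally controlled player passes through it.
; At BeginPlay it hides unless the game mode is Race_GameMode, otherwise snapping to the first transform in Checkpoint_Manager_BP.
; Each local overlap advances the count, reports progress to the manager and teleports the ring onward, or ends the race and deactivates it.
; A Tick-driven cooldown blocks repeat overlaps after each move.
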(event OnComponentBeginOverlap(CylinderCollider)
  (params (OverlappedComponent :type Primitive%20Component%20Object%20Reference) (OtherActor :type Actor%20Object%20Reference) (OtherComp :type Primitive%20Component%20Object%20Reference) (OtherBodyIndex :type Integer) (bFromSweep :type Boolean) (SweepResult :type Hit%20Result%20Structure%20%28by%20ref%29))
  ;[1 0.3102 0.9051] Begin Overlap
  ;;[1 1 1] If the buffer time is above 0, we don't register collision
  (if (<= (Variables|Default|GetcurrentBufferDelayTime) 0.0)
    (bind _asplayer_character (Utilities|Casting|CastToPlayerCharacter OtherActor))
    ;;[1 1 1] If the player that hit this checkpoint is controlled locally, we update our current checkpoint number
    (if (Pawn|IsLocallyControlled _asplayer_character)
      (Variables|Default|SetcurrentCheckpointNum (+ (Variables|Default|GetcurrentCheckpointNum) 1))
      (bind _israceover (CallFunction|IsRaceOver))
      (if _israceover
        ;;[1 1 1] If the player reached the last checkpoint, we disable this checkpoint and end the race
        (Default|EndRace (Variables|Default|GetcheckpointManagerRef) _asplayer_character)
        (CallFunction|SetCheckpointActive false)
        (else
          ;;[1 1 1] If this isn't the last checkpoint location, we move to the next location and update the player's progress
          (CallFunction|MovetoNextPos)
          (Development|PrintString "CHECKPOINT RING: Before update player progress" true true "(R=1.000000,G=0.000000,B=0.052997,A=1.000000)" 1e+01)
          (Default|UpdatePlayerProgress (Variables|Default|GetcheckpointManagerRef) _asplayer_character (Variables|Default|GetcurrentCheckpointNum))
          (Development|PrintString "CHECKPOINT RING: After update player progress" true true "(R=1.000000,G=0.000000,B=0.052997,A=1.000000)" 1e+01))))))

(event EventBeginPlay
  ;[0.3102 1 0.2353] Begin Play
  (Utilities|Casting|CastToRace_GameMode (Variables|/Script/Engine.GameStateBase|GetAuthorityGameMode (Game|GetGameState))
    (:then
      (CallFunction|GetCheckpointManager)
      ;;[1 1 1] Getting a reference to the player on this client
      (Variables|Default|SetclientPlayer (Game|GetPlayerController 0))
      (CallFunction|MovetoFirstPos))
    (:CastFailed
      (Development|SetHiddeninGame (Variables|Default|GetCylinderCollider) true true))))

(event EventTick
  (params (DeltaSeconds :type Float%20%28single-precision%29))
  ;[1 0.1973 0.2272] Tick
  ;;[1 1 1] Counting down the collision buffer so we can check for collision again
  (if (> (Variables|Default|GetcurrentBufferDelayTime) 0.0)
    (Variables|Default|SetcurrentBufferDelayTime (- (Variables|Default|GetcurrentBufferDelayTime) DeltaSeconds))))

(fn ConstructionScript)

(fn SetCheckpointActive
  (params (isActive :type Boolean))
  (Components|Activation|SetActive (Variables|Default|GetCylinderCollider) isActive true)
  (Development|SetHiddeninGame (Variables|Default|GetCylinderCollider) (not isActive) true))

(fn OnRepNeedstobeDisabled
  (Networking|SwitchHasAuthority
    (:Remote
      (Development|PrintString "Disabled Checkpoint" true true "(R=0.000000,G=0.660000,B=1.000000,A=1.000000)" 1e+01)
      (CallFunction|SetCheckpointActive false)
      (CallFunction|SetCheckpointActive (Variables|Default|GetnextCheckpoint) true))))

(fn GetCheckpointManager
  ;[1 1 1] Finding the first Checkpoint Manager BP actor in the level and setting it as our reference
  (bind _outactors (Actor|GetAllActorsOfClass "/Game/GameModes/Race/Checkpoint_Manager_BP.Checkpoint_Manager_BP_C"))
  (if (> (Utilities|Array|Length _outactors) 0)
    (Variables|Default|SetcheckpointManagerRef (Utilities|Array|Get(acopy) _outactors))))

(fn MovetoFirstPos
  (bind _checkpointmanagerref (Variables|Default|GetcheckpointManagerRef))
  (bind _checkpointtransforms (Variables|/Game/GameModes/Race/Checkpoint_Manager_BP.Checkpoint_Manager_BP_C|GetcheckpointTransforms _checkpointmanagerref))
  (bind _output (Utilities|Array|Get(acopy) _checkpointtransforms))
  (bind (_location _rotation _scale) (Math|Transform|BreakTransform _output))
  (Transformation|SetActorLocation _location false true)
  (Transformation|SetActorRotation _rotation)
  (Transformation|SetActorScale3D _scale))

(fn MovetoNextPos
  (bind _checkpointmanagerref (Variables|Default|GetcheckpointManagerRef))
  (bind _currentcheckpointnum (Variables|Default|GetcurrentCheckpointNum))
  (bind _checkpointtransforms (Variables|/Game/GameModes/Race/Checkpoint_Manager_BP.Checkpoint_Manager_BP_C|GetcheckpointTransforms _checkpointmanagerref))
  (bind _output (Utilities|Array|Get(acopy) _checkpointtransforms _currentcheckpointnum))
  (bind (_location _rotation _scale) (Math|Transform|BreakTransform _output))
  (Transformation|SetActorLocation _location false true)
  (Transformation|SetActorRotation _rotation)
  (Transformation|SetActorScale3D _scale)
  (Variables|Default|SetcurrentBufferDelayTime (Variables|Default|GetcollisionBufferDelay)))

(fn IsRaceOver
  (return (not (< (Variables|Default|GetcurrentCheckpointNum) (Utilities|Array|Length (Variables|/Game/GameModes/Race/Checkpoint_Manager_BP.Checkpoint_Manager_BP_C|GetcheckpointTransforms (Variables|Default|GetcheckpointManagerRef)))))))