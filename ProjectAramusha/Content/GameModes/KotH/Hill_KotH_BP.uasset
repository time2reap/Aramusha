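; Hill actor for the King of the Hill mode that awards points to players standing inside its capture ring while active.
; An authority-only activation event shows the ring, and overlap events maintain the pool of players inside.
; A countdown in event Tick periodically gives every pooled player points through the game mode, using its settings.
; When its ticks run out, the hill resets, hides and clears the game mode's active-hill flag.
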(event OnComponentBeginOverlap(CaptureRing)
  (params (OverlappedComponent :type Primitive%20Component%20Object%20Reference) (OtherActor :type Actor%20Object%20Reference) (OtherComp :type Primitive%20Component%20Object%20Reference) (OtherBodyIndex :type Integer) (bFromSweep :type Boolean) (SweepResult :type Hit%20Result%20Structure%20%28by%20ref%29))
  (bind _asplayer_character (Utilities|Casting|CastToPlayerCharacter OtherActor))
  (Utilities|Array|AddUnique (Variables|Default|GetPlayerPool) _asplayer_character))

(event OnComponentEndOverlap(CaptureRing)
  (params (OverlappedComponent :type Primitive%20Component%20Object%20Reference) (OtherActor :type Actor%20Object%20Reference) (OtherComp :type Primitive%20Component%20Object%20Reference) (OtherBodyIndex :type Integer))
  (bind _asplayer_character (Utilities|Casting|CastToPlayerCharacter OtherActor))
  (Utilities|Array|RemoveItem (Variables|Default|GetPlayerPool) _asplayer_character))

(event Custom|Activate%20Hill
  (bind _capturering (Variables|Default|GetCaptureRing))
  (Networking|SwitchHasAuthority
    (:Authority
      (if (not (Variables|Default|GetActive))
        (Variables|Default|SetActive true)
        (Components|Activation|SetActive _capturering true true)
        (Development|SetHiddeninGame _capturering false true)))))

(event EventBeginPlay
  (bind _askot_h_game_mode (Utilities|Casting|CastToKotH_GameMode (Game|GetGameMode)))
  (bind _output_get (Variables|Default|SetGameMode _askot_h_game_mode))
  (Variables|Default|SetTicksRemaining (Variables|/Game/GameModes/KotH/KotH_GameMode.KotH_GameMode_C|GetHillPoints _output_get))
  (Variables|Default|SettrTick (Variables|/Game/GameModes/KotH/KotH_GameMode.KotH_GameMode_C|GetTickTime _output_get))
  (Variables|Default|SetPoints (Variables|/Game/GameModes/KotH/KotH_GameMode.KotH_GameMode_C|GetPointsToGive _output_get)))

(event Collision|EventActorBeginOverlap
  (params (OtherActor :type Actor%20Object%20Reference)))

(event EventTick
  (params (DeltaSeconds :type Float%20%28single-precision%29))
  (if (Variables|Default|GetActive)
    (bind _output_get (Variables|Default|SettrTick (- (Variables|Default|GettrTick) DeltaSeconds)))
    (if (<= _output_get 0.0)
      (CallFunction|Tick))))

(fn ConstructionScript)

(fn Tick
  (bind _gamemode (Variables|Default|GetGameMode))
  (bind _capturering (Variables|Default|GetCaptureRing))
  (bind _result (Math|Integer|DecrementInt (Variables|Default|GetTicksRemaining))
    (:%20%20
      (Development|PrintString (Utilities|String|ToString(Integer) _result) true true "(R=1.000000,G=0.747449,B=0.000000,A=1.000000)")
      (for _array_element (Variables|Default|GetPlayerPool)
        (Default|GivePoints _gamemode (Variables|Default|GetPoints) (Variables|/Game/PlayerCharacter/Blueprints/PlayerCharacter.PlayerCharacter_C|GetPlayerID _array_element)))
      (Variables|Default|SettrTick (Variables|/Game/GameModes/KotH/KotH_GameMode.KotH_GameMode_C|GetTickTime _gamemode))
      (if (<= (Variables|Default|GetTicksRemaining) 0)
        (Variables|Default|SetActive false)
        (Variables|Default|SetTicksRemaining (Variables|/Game/GameModes/KotH/KotH_GameMode.KotH_GameMode_C|GetHillPoints _gamemode))
        (Variables|/Game/GameModes/KotH/KotH_GameMode.KotH_GameMode_C|SetHillIsActive (Variables|Default|GetGameMode) false)
        (Development|SetHiddeninGame _capturering true true)
        (Components|Activation|SetActive _capturering false false)))))