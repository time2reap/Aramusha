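; Flamethrower hazard that cycles on timers through off, warm-up and on phases and kills players caught in its flame.
; BeginPlay caches the kill cylinder's scale and applies the starting phase from three bools, while Tick advances phases and toggles warm-up and fire particles.
; At phase changes, the cylinder shrinks to zero scale when off and is restored when on.
; Overlaps while on kill a living PlayerCharacter with forced ragdoll.
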(event OnComponentBeginOverlap(KillCylinder)
  (params (OverlappedComponent :type Primitive%20Component%20Object%20Reference) (OtherActor :type Actor%20Object%20Reference) (OtherComp :type Primitive%20Component%20Object%20Reference) (OtherBodyIndex :type Integer) (bFromSweep :type Boolean) (SweepResult :type Hit%20Result%20Structure%20%28by%20ref%29))
  ;[1 0.1974 0.1874] BeginOverlap
  (if (Variables|Default|GetisOn)
    (bind _asplayer_character (Utilities|Casting|CastToPlayerCharacter OtherActor))
    (if (not (Variables|/Game/PlayerCharacter/Blueprints/PlayerCharacter.PlayerCharacter_C|GetisDead _asplayer_character))
      (Default|KillPlayer _asplayer_character "NewEnumerator0" true))))

(event EventBeginPlay
  ;[0.4366 1 0.4713] Begin Play
  (Variables|Default|SetcolliderScale (Transformation|GetWorldScale (Variables|Default|GetKillCylinder)))
  ;;[1 1 1] If all bools are on, the flamethrower is set to OFF
  (if (Math|Boolean|ANDBoolean (Variables|Default|GetisOff) (Variables|Default|GetisWarmingUp) (Variables|Default|GetisOn))
    (Variables|Default|SetisWarmingUp false)
    (Variables|Default|SetisOn false))
  ;;[1 1 1] If all bools are off, the flamethrower is set to OFF
  (if (not (Math|Boolean|ANDBoolean (Variables|Default|GetisOff) (Variables|Default|GetisWarmingUp) (Variables|Default|GetisOn)))
    (Variables|Default|SetisOff true))
  (if (Variables|Default|GetisOff)
    (Components|Activation|Deactivate (Variables|Default|GetFireParticlesWarmup))
    (Components|Activation|Deactivate (Variables|Default|GetFireParticles))
    (Components|Activation|Deactivate (Variables|Default|GetKillCylinder))
    (elif (Variables|Default|GetisWarmingUp)
      (Components|Activation|Activate (Variables|Default|GetFireParticlesWarmup) false)
      (Components|Activation|Deactivate (Variables|Default|GetFireParticles))
      (Components|Activation|Deactivate (Variables|Default|GetKillCylinder))
      (elif (Variables|Default|GetisOn)
        (Components|Activation|Deactivate (Variables|Default|GetFireParticlesWarmup))
        (Components|Activation|Activate (Variables|Default|GetKillCylinder) false)
        (Components|Activation|Activate (Variables|Default|GetFireParticles) false)))))

(event EventTick
  (params (DeltaSeconds :type Float%20%28single-precision%29))
  (bind _offtime (Variables|Default|GetoffTime))
  (bind _ontime (Variables|Default|GetonTime))
  (bind _warmuptime (Variables|Default|GetwarmupTime))
  ;[0.3642 0.4171 1] Tick
  (Variables|Default|SetcurrentTimer (+ (Variables|Default|GetcurrentTimer) DeltaSeconds))
  (if (Variables|Default|GetisOff)
    (if (>= (Variables|Default|GetcurrentTimer) _offtime)
      (Variables|Default|SetcurrentTimer (- (Variables|Default|GetcurrentTimer) _offtime))
      (Variables|Default|SetisOff false)
      (Variables|Default|SetisWarmingUp true)
      (Components|Activation|Activate (Variables|Default|GetFireParticlesWarmup) false))
    (elif (Variables|Default|GetisWarmingUp)
      (if (>= (Variables|Default|GetcurrentTimer) _warmuptime)
        (Variables|Default|SetcurrentTimer (- (Variables|Default|GetcurrentTimer) _warmuptime))
        (Variables|Default|SetisWarmingUp false)
        (Variables|Default|SetisOn true)
        (Components|Activation|Deactivate (Variables|Default|GetFireParticlesWarmup))
        (Components|Activation|Activate (Variables|Default|GetKillCylinder) false)
        (Components|Activation|Activate (Variables|Default|GetFireParticles) false)
        (Transformation|SetWorldScale3D (Variables|Default|GetKillCylinder) (Variables|Default|GetcolliderScale)))
      (elif (Variables|Default|GetisOn)
        (if (>= (Variables|Default|GetcurrentTimer) _ontime)
          (Variables|Default|SetcurrentTimer (- (Variables|Default|GetcurrentTimer) _ontime))
          (Variables|Default|SetisOn false)
          (Variables|Default|SetisOff true)
          (Components|Activation|Deactivate (Variables|Default|GetFireParticles))
          (Components|Activation|Deactivate (Variables|Default|GetKillCylinder))
          (Transformation|SetWorldScale3D (Variables|Default|GetKillCylinder) "0, 0, 0"))))))

(fn ConstructionScript)