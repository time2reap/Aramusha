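; KillWall is a hazard wall that kills player characters on hit, optionally only when their speed exceeds a force threshold.
; Hit adds the other actor to an ignore list to suppress repeat hits, then clears the list after a delay for players.
; It also zeroes the player mesh's physics velocity.
; A clamped rebound vector is calculated from hit normal and speed, but is only printed, never applied.
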(event EventBeginPlay)

(event Collision|EventActorBeginOverlap
  (params (OtherActor :type Actor%20Object%20Reference)))

(event EventTick
  (params (DeltaSeconds :type Float%20%28single-precision%29)))

(event Collision|EventHit
  (params (MyComp :type Primitive%20Component%20Object%20Reference) (Other :type Actor%20Object%20Reference) (OtherComp :type Primitive%20Component%20Object%20Reference) (bSelfMoved :type Boolean) (HitLocation :type Vector :default "0, 0, 0") (HitNormal :type Vector :default "0, 0, 0") (NormalImpulse :type Vector :default "0, 0, 0") (Hit :type Hit%20Result%20Structure%20%28by%20ref%29))
  (bind _ignorelist (Variables|Default|GetIgnoreList))
  (bind _forcelimit (Variables|Default|GetForceLimit))
  (bind _returnvalue (* _forcelimit -1.0))
  (if (not (Utilities|Array|ContainsItem _ignorelist Other))
    (Utilities|Array|AddUnique _ignorelist Other)
    (bind _asplayer_character (Utilities|Casting|CastToPlayerCharacter Other))
    (bind _output_get (Variables|Default|SetReboundForce (Math|Vector|MakeVector (Math|Float|Clamp(Float) (.x (* (.normal Hit) (* (Variables|Default|GetBounceForce) (Math|Vector|VectorLength (Transformation|GetVelocity _asplayer_character))))) _returnvalue _forcelimit) (Math|Float|Clamp(Float) (.y (* (.normal Hit) (* (Variables|Default|GetBounceForce) (Math|Vector|VectorLength (Transformation|GetVelocity _asplayer_character))))) _returnvalue _forcelimit) (Math|Float|Clamp(Float) (.z (* (.normal Hit) (* (Variables|Default|GetBounceForce) (Math|Vector|VectorLength (Transformation|GetVelocity _asplayer_character))))) _returnvalue _forcelimit))))
    (Development|PrintString (Utilities|String|ToString(Vector) _output_get))
    (if (Variables|Default|GetRequiresForceToKill?)
      (if (> (Math|Vector|VectorLength (Transformation|GetVelocity _asplayer_character)) (Variables|Default|GetForceToKill))
        (Default|KillPlayer _asplayer_character (Game|GetPlayerController (Variables|/Game/PlayerCharacter/Blueprints/PlayerCharacter.PlayerCharacter_C|GetPlayerID _asplayer_character)) :!label _label))
      (else
        (goto _label)))
    (Class|PrimitiveComponent|SetAllPhysicsLinearVelocity (Variables|/Script/Engine.Character|GetMesh _asplayer_character) "0, 0, 0" false)
    (Utilities|FlowControl|Delay 1.0)
    (Utilities|Array|Clear (Variables|Default|GetIgnoreList))))

(fn ConstructionScript)

(fn ResetIgnoreList
  (Utilities|Array|Clear (Variables|Default|GetIgnoreList)))