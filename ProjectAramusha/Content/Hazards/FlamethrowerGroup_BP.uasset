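; Timed hazard of four flamethrowers that kills a living player with forced ragdoll on entering its shared KillBox while firing.
; Tick accumulates time to cycle through off, warmup and on phases, toggling warmup and fire particle sets; BeginPlay always sets IsOff.
; The KillBox shrinks to zero scale when fire stops and regains its saved scale on ignition, alongside activation toggles.
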(event OnComponentBeginOverlap(KillBox)
  (params (OverlappedComponent :type Primitive%20Component%20Object%20Reference) (OtherActor :type Actor%20Object%20Reference) (OtherComp :type Primitive%20Component%20Object%20Reference) (OtherBodyIndex :type Integer) (bFromSweep :type Boolean) (SweepResult :type Hit%20Result%20Structure%20%28by%20ref%29))
  ;[1 0.1667 0.1667] BeginOverlap
  (if (Variables|Default|GetisOn)
    (bind _asplayer_character (Utilities|Casting|CastToPlayerCharacter OtherActor))
    (if (not (Variables|/Game/PlayerCharacter/Blueprints/PlayerCharacter.PlayerCharacter_C|GetisDead _asplayer_character))
      (Default|KillPlayer _asplayer_character "NewEnumerator0" true))))

(event EventBeginPlay
  ;[0.4366 1 0.4713] Begin Play
  (Variables|Default|SetcolliderScale (Transformation|GetWorldScale (Variables|Default|GetKillBox)))
  ;;[1 1 1] If all bools are on, the flamethrower is set to OFF
  (if (Math|Boolean|ANDBoolean (Variables|Default|GetisOff) (Variables|Default|GetisWarmingUp) (Variables|Default|GetisOn))
    (Variables|Default|SetisWarmingUp false)
    (Variables|Default|SetisOn false))
  ;;[1 1 1] If all bools are off, the flamethrower is set to OFF
  (if (not (Math|Boolean|ANDBoolean (Variables|Default|GetisOff) (Variables|Default|GetisWarmingUp) (Variables|Default|GetisOn)))
    (Variables|Default|SetisOff true))
  (if (Variables|Default|GetisOff)
    (Components|Activation|Deactivate (Variables|Default|GetKillBox))
    (CallFunction|ToggleWarmupParticles false)
    (CallFunction|ToggleFireParticles false)
    (elif (Variables|Default|GetisWarmingUp)
      (Components|Activation|Deactivate (Variables|Default|GetKillBox))
      (CallFunction|ToggleWarmupParticles true)
      (CallFunction|ToggleFireParticles false)
      (elif (Variables|Default|GetisOn)
        (Components|Activation|Activate (Variables|Default|GetKillBox) false)
        (CallFunction|ToggleWarmupParticles false)
        (CallFunction|ToggleFireParticles true)))))

(event EventTick
  (params (DeltaSeconds :type Float%20%28single-precision%29))
  (bind _offtime (Variables|Default|GetoffTime))
  (bind _ontime (Variables|Default|GetonTime))
  (bind _warmuptime (Variables|Default|GetwarmupTime))
  ;[0.3642 0.4171 1] Tick
  (Variables|Default|SetcurrentTimer (+ (Variables|Default|GetcurrentTimer) DeltaSeconds))
  (if (Variables|Default|GetisOff)
    (if (>= (Variables|Default|GetcurrentTimer) _offtime)
      (Variables|Default|SetcurrentTimer (- (Variables|Default|GetcurrentTimer) _offtime))
      (Variables|Default|SetisOff false)
      (Variables|Default|SetisWarmingUp true)
      (CallFunction|ToggleWarmupParticles true))
    (elif (Variables|Default|GetisWarmingUp)
      (if (>= (Variables|Default|GetcurrentTimer) _warmuptime)
        (Variables|Default|SetcurrentTimer (- (Variables|Default|GetcurrentTimer) _warmuptime))
        (Variables|Default|SetisWarmingUp false)
        (Variables|Default|SetisOn true)
        (CallFunction|ToggleWarmupParticles false)
        (CallFunction|ToggleFireParticles true))
      (elif (Variables|Default|GetisOn)
        (if (>= (Variables|Default|GetcurrentTimer) _ontime)
          (Variables|Default|SetcurrentTimer (- (Variables|Default|GetcurrentTimer) _ontime))
          (Variables|Default|SetisOn false)
          (Variables|Default|SetisOff true)
          (CallFunction|ToggleFireParticles false))))))

(fn ConstructionScript)

(fn ToggleWarmupParticles
  (params (activate :type Boolean))
  (if activate
    (Components|Activation|Activate (Variables|Default|GetFireParticlesWarmup1) false)
    (Components|Activation|Activate (Variables|Default|GetFireParticlesWarmup2) false)
    (Components|Activation|Activate (Variables|Default|GetFireParticlesWarmup3) false)
    (Components|Activation|Activate (Variables|Default|GetFireParticlesWarmup4) false)
    (else
      (Components|Activation|Deactivate (Variables|Default|GetFireParticlesWarmup1))
      (Components|Activation|Deactivate (Variables|Default|GetFireParticlesWarmup2))
      (Components|Activation|Deactivate (Variables|Default|GetFireParticlesWarmup3))
      (Components|Activation|Deactivate (Variables|Default|GetFireParticlesWarmup4)))))

(fn ToggleFireParticles
  (params (activate :type Boolean))
  (if activate
    (Components|Activation|Activate (Variables|Default|GetFireParticles1) false)
    (Components|Activation|Activate (Variables|Default|GetFireParticles2) false)
    (Components|Activation|Activate (Variables|Default|GetFireParticles3) false)
    (Components|Activation|Activate (Variables|Default|GetFireParticles4) false)
    (Components|Activation|Activate (Variables|Default|GetKillBox) true)
    (Transformation|SetWorldScale3D (Variables|Default|GetKillBox) (Variables|Default|GetcolliderScale))
    (else
      (Components|Activation|Deactivate (Variables|Default|GetFireParticles1))
      (Components|Activation|Deactivate (Variables|Default|GetFireParticles2))
      (Components|Activation|Deactivate (Variables|Default|GetFireParticles3))
      (Components|Activation|Deactivate (Variables|Default|GetFireParticles4))
      (Components|Activation|Deactivate (Variables|Default|GetKillBox))
      (Transformation|SetWorldScale3D (Variables|Default|GetKillBox) "0, 0, 0"))))