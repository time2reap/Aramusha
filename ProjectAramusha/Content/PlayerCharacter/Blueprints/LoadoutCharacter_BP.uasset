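; LoadoutCharacter_BP is a player character for the loadout game mode that gives its player a loadout UI.
; On BeginPlay it adds itself uniquely to the Loadout_GameMode's CurrentPlayers list.
; It then creates a Loadout_Widget owned by the player controller matching its PID, passes itself as the Character, adds it to the viewport and stores it as PlayerWidget.
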(event EventBeginPlay
  (bind _asloadout_game_mode (Utilities|Casting|CastToLoadout_GameMode (Game|GetGameMode))
    (:then
      (Utilities|Array|AddUnique (Variables|/Game/GameModes/Loadout_GameMode.Loadout_GameMode_C|GetCurrentPlayers _asloadout_game_mode) self))
    (:CastFailed
      _))
  (bind _returnvalue (UserInterface|CreateWidget "/Game/Lobby/Loadout_Widget.Loadout_Widget_C" (Utilities|GetPlayerControllerbyID (Variables|Default|GetPID)) self))
  (UserInterface|Viewport|AddtoViewport _returnvalue 0)
  (Variables|Default|SetPlayerWidget _returnvalue))

(event Collision|EventActorBeginOverlap
  (params (OtherActor :type Actor%20Object%20Reference)))

(event EventTick
  (params (DeltaSeconds :type Float%20%28single-precision%29)))

(fn ConstructionScript)