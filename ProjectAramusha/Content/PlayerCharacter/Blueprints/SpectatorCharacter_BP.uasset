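; Spectator character that shows a player the level overview and handles spawning that player's playable character.
; SetupSC runs its logic on the remote side, adding the spectator widget, switching the view to the level camera and setting UI-only input.
; SpawnPlayerChar_Net passes the player's abilities, color and name from the GameInstance's PlayerInfoList to CoreGameState's SpawnPlayerRPC, using test defaults when the PID has no entry.
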(event Custom|SetupSC
  (Networking|SwitchHasAuthority
    (:Remote
      (bind _returnvalue (UserInterface|CreateWidget "/Game/GameModes/Spectator_Widget.Spectator_Widget_C" (Variables|Default|GetPlayerController) self))
      (bind _output_get (Variables|Default|SetPlayerWidget _returnvalue))
      (UserInterface|Viewport|AddtoViewport _output_get 0)
      (bind _outactors (Actor|GetAllActorsOfClass "/Game/Levels/LevelCamera_Blueprint.LevelCamera_Blueprint_C"))
      (Utilities|IsValid (Variables|Default|GetPlayerController)
        (:Is%20Valid
          _)
        (:Is%20Not%20Valid
          (Networking|SwitchHasAuthority
            (:Remote
              (bind _asplayer_character_controller (Utilities|Casting|CastToPlayerCharacterController (Game|GetPlayerController 0)))
              (Variables|Default|SetPlayerController _asplayer_character_controller)))))
      (Game|Player|SetViewTargetwithBlend (Variables|Default|GetPlayerController) (Utilities|Array|Get(acopy) _outactors) 0.0 "VTBlend_Linear" 0.0 true)
      (Input|SetInputModeUIOnly (Variables|Default|GetPlayerController) (Variables|Default|GetPlayerWidget) "DoNotLock"))))

(event Custom|SpawnPlayerChar_Net
  (bind _pid (Variables|Default|GetPID))
  (bind _gameinstance (Variables|Default|GetGameInstance))
  (bind _playercontroller (Variables|Default|GetPlayerController))
  (bind _playerinfolist (Variables|/Game/GameBP/Main_GameInstance.Main_GameInstance_C|GetPlayerInfoList _gameinstance))
  (bind _output (Utilities|Array|Get(acopy) _playerinfolist _pid))
  (Utilities|IsValid _gameinstance
    (:Is%20Valid
      (if (Utilities|Array|IsValidIndex _playerinfolist _pid)
        (Default|SpawnPlayerRPC (Variables|Default|GetCoreGameState) (.ability1 _output) (.ability2 _output) _pid (.primarycolor _output) (.displayname _output) (Variables|Default|GetPlayerController))
        (else
          (Utilities|IsValid _playercontroller
            (:Is%20Valid
              (Default|SpawnPlayerRPC (Variables|Default|GetCoreGameState) "/Game/Abilities/Dash_A.Dash_A_C" "/Game/Abilities/OmegaPunch_A.OmegaPunch_A_C" (Variables|Default|GetPID) "(R=0.463542,G=0.000000,B=0.022826,A=1.000000)" "Test Player" _playercontroller))
            (:Is%20Not%20Valid
              (Development|PrintString "WARNING: FAILED TO CREATE PLAYER" true true "(R=1.000000,G=0.856228,B=0.000000,A=1.000000)" 5.0))))))))

(fn ConstructionScript
  (bind _asmain_game_instance (Utilities|Casting|CastToMain_GameInstance (Game|GetGameInstance)))
  (Variables|Default|SetGameInstance _asmain_game_instance)
  (bind _ascore_game_state (Utilities|Casting|CastToCoreGameState (Game|GetGameState)))
  (Variables|Default|SetCoreGameState _ascore_game_state))