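; Main menu character that prepares the local save and opens the menu UI when possessed.
; On authority, possession loads the Player1 save through Main_GameInstance, or creates and writes a new GameSaveData if none exists.
; SetupMainMenu then adds MainMenu_Widget, shows the cursor and sets UI-only input, focusing the separate PlayerWidget variable.
; The construction script caches the game instance and CoreGameState.
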(event Custom|SetupMainMenu
  (params (Controller :type Controller%20Object%20Reference))
  (bind _asplayer_character_controller (Utilities|Casting|CastToPlayerCharacterController Controller))
  (Variables|Default|SetPlayerController _asplayer_character_controller)
  (bind _asmain_game_instance (Utilities|Casting|CastToMain_GameInstance (Game|GetGameInstance)))
  (Variables|Default|SetGameInstance _asmain_game_instance)
  (bind _returnvalue (UserInterface|CreateWidget "/Game/MainMenu/MainMenu_Widget.MainMenu_Widget_C" (Variables|Default|GetPlayerController)))
  (UserInterface|Viewport|AddtoViewport _returnvalue 0)
  (Variables|/Script/Engine.PlayerController|SetbShowMouseCursor (Variables|Default|GetPlayerController) true)
  (Input|SetInputModeUIOnly (Variables|Default|GetPlayerController) (Variables|Default|GetPlayerWidget) "DoNotLock"))

(event EventPossessed
  (params (NewController :type Controller%20Object%20Reference))
  (Networking|SwitchHasAuthority
    (:Authority
      (bind _returnvalue (SaveGame|DoesSaveGameExist "Player1"))
      (if _returnvalue
        (bind _asmain_game_instance (Utilities|Casting|CastToMain_GameInstance (Game|GetGameInstance)))
        (Default|LoadLocalSaveData _asmain_game_instance)
        (else
          (bind _returnvalue_2 (SaveGame|CreateSaveGameObject "/Game/GameBP/GameSaveData.GameSaveData_C"))
          (bind _asmain_game_instance_2 (Utilities|Casting|CastToMain_GameInstance (Game|GetGameInstance)))
          (bind _output_get (Variables|/Game/GameBP/Main_GameInstance.Main_GameInstance_C|SetGameSave _asmain_game_instance_2 _returnvalue_2))
          (SaveGame|SaveGametoSlot _output_get "Player1")))
      (CallFunction|SetupMainMenu NewController))))

(fn ConstructionScript
  (bind _asmain_game_instance (Utilities|Casting|CastToMain_GameInstance (Game|GetGameInstance)))
  (Variables|Default|SetGameInstance _asmain_game_instance)
  (bind _ascore_game_state (Utilities|Casting|CastToCoreGameState (Game|GetGameState)))
  (Variables|Default|SetCoreGameState _ascore_game_state))