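; RadialForce_BP is an ability helper actor that launches overlapping players and physics objects straight up, despite its radial name.
; On BeginPlay it deactivates its collision sphere, waits for a delay, draws a debug sphere, reactivates the collision and sets a short lifespan.
; Overlaps apply a fixed upward velocity-change impulse to the CharacterMovement of Player-tagged characters, or to other components that simulate physics.
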(event OnComponentBeginOverlap(CollisionSphere)
  (params (OverlappedComponent :type Primitive%20Component%20Object%20Reference) (OtherActor :type Actor%20Object%20Reference) (OtherComp :type Primitive%20Component%20Object%20Reference) (OtherBodyIndex :type Integer) (bFromSweep :type Boolean) (SweepResult :type Hit%20Result%20Structure%20%28by%20ref%29))
  (if (Actor|ActorHasTag OtherActor "Player")
    (bind _asplayer_character (Utilities|Casting|CastToPlayerCharacter OtherActor))
    (Physics|AddImpulse (Variables|/Script/Engine.Character|GetCharacterMovement _asplayer_character) "0, 0,5000.000000" true)
    (elif (Physics|IsSimulatingPhysics OtherComp "None")
      (Physics|AddImpulse OtherComp "0, 0,5000.000000" "None" true))))

(event EventBeginPlay
  (Components|Activation|SetActive (Variables|Default|GetCollisionSphere) false false)
  (Utilities|FlowControl|Delay (Variables|Default|GetDelay))
  (Rendering|Debug|DrawDebugSphere (Transformation|GetWorldLocation (Variables|Default|GetDefaultSceneRoot)) (Variables|/Script/Engine.SphereComponent|GetSphereRadius (Variables|Default|GetCollisionSphere)) 30 "(R=0.000000,G=0.025125,B=1.000000,A=1.000000)" 0.5 1.0)
  (Components|Activation|SetActive (Variables|Default|GetCollisionSphere) true true)
  (Actor|SetLifeSpan 0.25))

(event EventTick
  (params (DeltaSeconds :type Float%20%28single-precision%29)))

(fn ConstructionScript)