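; Force push ability actor that, after a delay, activates a sphere trigger for a limited lifetime and draws a debug sphere.
; Overlapping Player-tagged characters and physics-simulating "Forceable" actors receive a velocity-change impulse away from the center, scaled up with distance relative to the radius.
; An ignore list, filled on push and on overlap exit, is checked to prevent repeat hits and optionally exclude the user.
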(event OnComponentBeginOverlap(CollisionSphere)
  (params (OverlappedComponent :type Primitive%20Component%20Object%20Reference) (OtherActor :type Actor%20Object%20Reference) (OtherComp :type Primitive%20Component%20Object%20Reference) (OtherBodyIndex :type Integer) (bFromSweep :type Boolean) (SweepResult :type Hit%20Result%20Structure%20%28by%20ref%29))
  (if (Actor|ActorHasTag OtherActor "Player")
    (bind _valid (CallFunction|ValidateTarget OtherActor))
    (if _valid
      (bind _asplayer_character (Utilities|Casting|CastToPlayerCharacter OtherActor))
      (bind _force (CallFunction|CalculateForce _asplayer_character))
      (Physics|AddImpulse (Variables|/Script/Engine.Character|GetCharacterMovement _asplayer_character) _force true)
      (Utilities|Array|AddUnique (Variables|Default|GetIgnoreList) _asplayer_character))
    (else
      (bind _valid_2 (CallFunction|ValidateTarget OtherActor))
      (if (Math|Boolean|ANDBoolean (Actor|ActorHasTag OtherActor "Forceable") (Class|SceneComponent|IsAnySimulatingPhysics (Variables|/Script/Engine.Actor|GetRootComponent OtherActor)) _valid_2)
        (bind _force_2 (CallFunction|CalculateForce OtherActor))
        (Physics|AddImpulse OtherComp _force_2 "None" true)
        (Utilities|Array|AddUnique (Variables|Default|GetIgnoreList) (Components|GetOwner OtherComp))))))

(event OnComponentEndOverlap(CollisionSphere)
  (params (OverlappedComponent :type Primitive%20Component%20Object%20Reference) (OtherActor :type Actor%20Object%20Reference) (OtherComp :type Primitive%20Component%20Object%20Reference) (OtherBodyIndex :type Integer))
  (Utilities|Array|AddUnique (Variables|Default|GetIgnoreList) OtherActor))

(event EventBeginPlay
  (Components|Activation|SetActive (Variables|Default|GetCollisionSphere) false false)
  (Components|Sphere|SetSphereRadius (Variables|Default|GetCollisionSphere) (Variables|Default|GetRadius) true)
  (if (Variables|Default|GetCanAffectSelf)
    _
    (else
      (Utilities|Array|AddUnique (Variables|Default|GetIgnoreList) (Variables|Default|GetUser))))
  (Utilities|FlowControl|Delay (Variables|Default|GetDelay))
  (Rendering|Debug|DrawDebugSphere (Transformation|GetWorldLocation (Variables|Default|GetDefaultSceneRoot)) (Variables|Default|GetRadius) 30 "(R=0.000000,G=0.025125,B=1.000000,A=1.000000)" 0.5 1.0)
  (Components|Activation|SetActive (Variables|Default|GetCollisionSphere) true true)
  (Actor|SetLifeSpan (Variables|Default|GetLifetime)))

(event EventTick
  (params (DeltaSeconds :type Float%20%28single-precision%29)))

(fn ConstructionScript)

(fn CalculateForce
  (params (Actor :type Actor%20Object%20Reference))
  (bind _returnvalue (Transformation|GetActorLocation Actor))
  (bind _self self)
  (bind _returnvalue_2 (Transformation|GetActorLocation _self))
  (bind _returnvalue_3 (- _returnvalue _returnvalue_2))
  ;[1 0 0.03849] Looping through all hit actors
  (return (* (Math|Vector|Normalize _returnvalue_3) (* (Variables|Default|GetForce) (/ (Math|Vector|VectorLength _returnvalue_3) (Variables|Default|GetRadius))))))

(fn ValidateTarget
  (params (Target :type Object%20Object%20Reference))
  (if (Variables|Default|GetCanAffectSelf)
    _
    (elif (== Target (Variables|Default|GetUser))
      (return false)
      (else
        _)))
  (bind _array_element (Utilities|Array|ForEachLoopwithBreak (Variables|Default|GetIgnoreList) :!label _label)
    (:LoopBody
      (if (== _array_element Target)
        (LocalVariables|SetValidTarget false)
        (goto _label Break)))
    (:Completed
      (return (LocalVariables|GetValidTarget)))))