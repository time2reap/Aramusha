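; Short-lived hitbox actor for the Omega Punch ability that knocks struck players along its forward vector, optionally ragdolling them.
; It gathers initial overlaps and processes them after a brief delay, while a begin-overlap handler catches players entering during the enabled window.
; A hit applies an RPC impulse, spawns a particle near the owner, fires a radial force, notifies the ability and destroys the actor.
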(event OnComponentBeginOverlap(HitBox)
  (params (OverlappedComponent :type Primitive%20Component%20Object%20Reference) (OtherActor :type Actor%20Object%20Reference) (OtherComp :type Primitive%20Component%20Object%20Reference) (OtherBodyIndex :type Integer) (bFromSweep :type Boolean) (SweepResult :type Hit%20Result%20Structure%20%28by%20ref%29))
  (if (Variables|Default|GetEnabled)
    (bind _valid (CallFunction|CheckHitList OtherActor))
    (if _valid
      (Utilities|Array|Add (Variables|Default|GetHitList) OtherActor)
      (bind _asplayer_character (Utilities|Casting|CastToPlayerCharacter OtherActor))
      (Variables|Default|SetEnabled false)
      (Default|RPCAddImpulsetoPlayer _asplayer_character (* (Transformation|GetActorForwardVector) (Variables|Default|GetHitForce)) true "0, 0, 0" (Variables|Default|GetUseRagdoll) "None" false)
      (CallFunction|RPCSpawnParticle)
      (Class|RadialForceComponent|FireImpulse (Variables|Default|GetRadialForce))
      (Default|PunchLanded (Variables|Default|GetmyAbility))
      (Actor|DestroyActor))))

(event Custom|RPC%20Spawn%20Particle
  ;[1 1 1] Particles
  (Effects|SpawnEmitteratLocation "/Game/InfinityBladeEffects/Effects/FX_Skill_TeleCharge/Omega_Punch_Hit_Particle.Omega_Punch_Hit_Particle" (+ (+ (Transformation|GetActorLocation (Variables|Default|GetOwnerActor)) (* (Transformation|GetActorForwardVector) 3e+01)) "0, 0,40.000000") "0, 0, 0" "3.000000,3.000000,3.000000"))

(event EventBeginPlay
  (Collision|IgnoreActorwhenMoving (Variables|Default|GetHitBox) (Variables|Default|GetOwnerActor) true)
  (for _array_element (Collision|GetOverlappingActors (Variables|Default|GetHitBox) "/Game/PlayerCharacter/Blueprints/PlayerCharacter.PlayerCharacter_C" :!class /Script/Engine.PrimitiveComponent)
    (if (and (!= _array_element (Variables|Default|GetOwnerActor)) (Utilities|Array|ContainsItem (Variables|Default|GetHitList) _array_element))
      (Utilities|Array|Add (Variables|Default|GetHitList) 0)))
  (Utilities|FlowControl|Delay 0.2)
  (for _array_element_2 (Variables|Default|GetHitList)
    (bind _asplayer_character (Utilities|Casting|CastToPlayerCharacter _array_element_2))
    (Variables|Default|SetEnabled false)
    (Default|RPCAddImpulsetoPlayer _asplayer_character (* (Transformation|GetActorForwardVector) (Variables|Default|GetHitForce)) false "0, 0, 0" (Variables|Default|GetUseRagdoll) "None" true)
    (Variables|Default|SetActivated true)
    (CallFunction|RPCSpawnParticle))
  (if (and (not (Variables|Default|GetEnabled)) (Variables|Default|GetActivated))
    (Class|RadialForceComponent|FireImpulse (Variables|Default|GetRadialForce))
    (Default|PunchLanded (Variables|Default|GetmyAbility))
    (Actor|DestroyActor)))

(fn ConstructionScript)

(fn CheckHitList
  (params (Other%20Actor :type Actor%20Object%20Reference))
  (if (== Other%20Actor (Variables|Default|GetOwnerActor))
    (LocalVariables|Setreturn false)
    (else
      (for _array_element (Variables|Default|GetHitList)
        (if (or (== Other%20Actor _array_element) (== Other%20Actor (Actor|GetParentActor)))
          (LocalVariables|Setreturn false)
          (return (LocalVariables|Getreturn))))))
  (return (LocalVariables|Getreturn)))