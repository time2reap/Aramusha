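; Timed gravity well ability actor that pulls player characters and physics objects toward its center, playing a sound on spawn.
; Sphere overlaps maintain lists of affected players and simulating primitives, which receive impulses every Tick.
; Pull grows with radius over distance, using separate min/max forces for players (velocity change) and objects.
; Actor scale fades in and out over its lifespan, resizing the sphere, which is debug-drawn each frame.
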(event OnComponentBeginOverlap(CollisionSphere)
  (params (OverlappedComponent :type Primitive%20Component%20Object%20Reference) (OtherActor :type Actor%20Object%20Reference) (OtherComp :type Primitive%20Component%20Object%20Reference) (OtherBodyIndex :type Integer) (bFromSweep :type Boolean) (SweepResult :type Hit%20Result%20Structure%20%28by%20ref%29))
  ;[1 1 1] If the hit object is a player character
  (bind _asplayer_character (Utilities|Casting|CastToPlayerCharacter OtherActor)
    (:then
      (if (not (Utilities|Array|ContainsItem (Variables|Default|GetaffectedPlayers) _asplayer_character))
        (Utilities|Array|AddUnique (Variables|Default|GetaffectedPlayers) _asplayer_character)))
    (:CastFailed
      ;[1 1 1] If the hit object is a physics primitive
      (if (Physics|IsSimulatingPhysics OtherComp "None")
        (if (not (Utilities|Array|ContainsItem (Variables|Default|GetaffectedPrimitives) OtherComp))
          (Utilities|Array|AddUnique (Variables|Default|GetaffectedPrimitives) OtherComp))))))

(event OnComponentEndOverlap(CollisionSphere)
  (params (OverlappedComponent :type Primitive%20Component%20Object%20Reference) (OtherActor :type Actor%20Object%20Reference) (OtherComp :type Primitive%20Component%20Object%20Reference) (OtherBodyIndex :type Integer))
  ;[1 1 1] If the player character was being affected, we remove it from our array
  (bind _asplayer_character (Utilities|Casting|CastToPlayerCharacter OtherActor))
  (if true
    (Utilities|Array|RemoveItem (Variables|Default|GetaffectedPlayers) _asplayer_character))
  ;[1 1 1] If the object hit was a physics object, we remove it from our array
  (if (Utilities|Array|ContainsItem (Variables|Default|GetaffectedPrimitives) OtherComp)
    (Utilities|Array|RemoveItem (Variables|Default|GetaffectedPrimitives) OtherComp)))

(event Custom|PlayGravitySound
  ;[0.6908 1 0.7043] Play Gravity Sound
  (Audio|SpawnSoundatLocation (Variables|Default|GetgravityWellSFX) (.Location (Math|Transform|BreakTransform (Transformation|GetActorTransform self))) "0, 0, 0" (Variables|Default|GetgravityWellSFXVolume) (Variables|Default|GetgravityWellSFXPitch) 0.08 0 0 false))

(event EventBeginPlay
  ;[1 1 1] Setting this gravity well to destroy itself when the duration is up
  (Actor|SetLifeSpan (Variables|Default|Getduration))
  (Transformation|SetActorScale3D "0, 0, 0")
  (CallFunction|PlayGravitySound))

(event EventTick
  (params (DeltaSeconds :type Float%20%28single-precision%29))
  (CallFunction|ChangeSphereScale DeltaSeconds)
  ;[1 1 1] Applying force to all of our physics primitives
  (for _array_element (Variables|Default|GetaffectedPrimitives)
    (bind _gravityforcevector (CallFunction|GetGravityForceVector (Transformation|GetWorldLocation _array_element) false))
    (Physics|AddImpulse _array_element _gravityforcevector "None" false))
  ;[1 1 1] Applying force to all of our characters
  (for _array_element_2 (Variables|Default|GetaffectedPlayers)
    (bind _gravityforcevector_2 (CallFunction|GetGravityForceVector (Transformation|GetActorLocation _array_element_2) true))
    (Physics|AddImpulse (Variables|/Script/Engine.Character|GetCharacterMovement _array_element_2) _gravityforcevector_2 true)))

(fn ConstructionScript)

(fn GetGravityForceVector
  (params (targetLocation :type Vector) (isPlayer :type Boolean))
  (bind _returnvalue (Transformation|GetActorLocation))
  (bind _returnvalue_2 (Transformation|GetActorLocation))
  (bind _returnvalue_3 (- _returnvalue targetLocation))
  (bind _returnvalue_4 (- _returnvalue_2 targetLocation))
  (if isPlayer
    (return (* (* (Math|Vector|Normalize _returnvalue_3) (+ (* (/ (Components|Sphere|GetScaledSphereRadius (Variables|Default|GetCollisionSphere)) (Math|Vector|VectorLength _returnvalue_3)) (- (Variables|Default|GetmaxPlayerForce) (Variables|Default|GetminPlayerForce))) (Variables|Default|GetminPlayerForce))) 1))
    (else
      (return (* (* (Math|Vector|Normalize _returnvalue_4) (+ (* (/ (Components|Sphere|GetScaledSphereRadius (Variables|Default|GetCollisionSphere)) (Math|Vector|VectorLength _returnvalue_4)) (- (Variables|Default|GetmaxObjectForce) (Variables|Default|GetminObjectForce))) (Variables|Default|GetminObjectForce))) 1)))))

(fn ChangeSphereScale
  (params (deltaTime :type Float%20%28single-precision%29))
  (Variables|Default|SetcurrentFadeTime (+ (Variables|Default|GetcurrentFadeTime) deltaTime))
  ;[1 1 1] If this object is fading in, we increase the scale
  (if (< (Variables|Default|GetcurrentFadeTime) (Variables|Default|GetfadeInTime))
    (Transformation|SetActorScale3D (* "1.000000,1.000000,1.000000" (/ (Variables|Default|GetcurrentFadeTime) (Variables|Default|GetfadeInTime))))
    (else
      ;[1 1 1] If this object is fading out, we decrease the scale
      (if (> (Variables|Default|GetcurrentFadeTime) (- (Variables|Default|Getduration) (Variables|Default|GetfadeOutTime)))
        (Transformation|SetActorScale3D (* "1.000000,1.000000,1.000000" (/ (- (Variables|Default|Getduration) (Variables|Default|GetcurrentFadeTime)) (Variables|Default|GetfadeOutTime))))
        (else
          ;[1 1 1] Otherwise this object has the default scale
          (Transformation|SetActorScale3D "1.000000,1.000000,1.000000")))))
  (Rendering|Debug|DrawDebugSphere (Transformation|GetActorLocation) (Components|Sphere|GetScaledSphereRadius (Variables|Default|GetCollisionSphere)) 16 "(R=1.000000,G=1.000000,B=1.000000,A=1.000000)" 0.0))