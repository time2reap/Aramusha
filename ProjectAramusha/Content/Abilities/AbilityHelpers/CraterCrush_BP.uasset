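; Crater Crush ability helper actor that launches players in a spherical area upward after a delay, then destroys itself.
; A radius-sized collision sphere keeps a pool of overlapping player characters, filtered by an ignore list and optional exclusion of the user.
; On activation it spawns an impact effect, sends launch RPCs to the pool, and calls each player's ragdoll RPC a moment later.
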(event OnComponentBeginOverlap(CollisionSphere)
  (params (OverlappedComponent :type Primitive%20Component%20Object%20Reference) (OtherActor :type Actor%20Object%20Reference) (OtherComp :type Primitive%20Component%20Object%20Reference) (OtherBodyIndex :type Integer) (bFromSweep :type Boolean) (SweepResult :type Hit%20Result%20Structure%20%28by%20ref%29))
  (Utilities|IsValid OtherActor
    (:Is%20Valid
      (bind _valid (CallFunction|ValidateTarget OtherActor))
      (if _valid
        (bind _asplayer_character (Utilities|Casting|CastToPlayerCharacter OtherActor))
        (Utilities|Array|AddUnique (Variables|Default|GetPlayerPool) _asplayer_character)))))

(event OnComponentEndOverlap(CollisionSphere)
  (params (OverlappedComponent :type Primitive%20Component%20Object%20Reference) (OtherActor :type Actor%20Object%20Reference) (OtherComp :type Primitive%20Component%20Object%20Reference) (OtherBodyIndex :type Integer))
  (bind _playerpool (Variables|Default|GetPlayerPool))
  (bind _asplayer_character (Utilities|Casting|CastToPlayerCharacter OtherActor))
  (if (Utilities|Array|ContainsItem _playerpool _asplayer_character)
    (Utilities|Array|RemoveItem _playerpool _asplayer_character)))

(event Custom|Activate
  (Effects|SpawnEmitteratLocation "/Game/InfinityBladeEffects/Effects/FX_Monsters/FX_Monster_Sentinel/P_Sentinel_LeapSlam_Impact.P_Sentinel_LeapSlam_Impact" (Transformation|GetWorldLocation (Variables|Default|GetCollisionSphere)) "0, 0, 0" "1.300000,1.300000,1.300000")
  (for _array_element (Variables|Default|GetPlayerPool)
    (Default|RPCLaunchPlayer _array_element (Math|Vector|MakeVector 0.0 0.0 (Variables|Default|GetLaunchDistance)) true false))
  (Utilities|FlowControl|Delay 0.35)
  (for _array_element_2 (Variables|Default|GetPlayerPool)
    (Default|RPCActivateRagdoll _array_element_2 false))
  (Actor|DestroyActor))

(event EventBeginPlay
  (Components|Activation|SetActive (Variables|Default|GetCollisionSphere) false false)
  (if (Variables|Default|GetCanAffectSelf)
    _
    (else
      (Utilities|Array|AddUnique (Variables|Default|GetIgnoreList) (Variables|Default|GetUser))))
  (Components|Activation|SetActive (Variables|Default|GetCollisionSphere) true true)
  (Utilities|FlowControl|Delay (Variables|Default|GetDelay))
  (CallFunction|Activate))

(fn ConstructionScript
  (Components|Sphere|SetSphereRadius (Variables|Default|GetCollisionSphere) (Variables|Default|GetRadius) true))

(fn ValidateTarget
  (params (Target :type Object%20Object%20Reference))
  (if (Variables|Default|GetCanAffectSelf)
    _
    (elif (== Target (Variables|Default|GetUser))
      (return false)
      (else
        _)))
  (bind _array_element (Utilities|Array|ForEachLoopwithBreak (Variables|Default|GetIgnoreList) :!label _label)
    (:LoopBody
      (if (== _array_element Target)
        (LocalVariables|SetValidTarget false)
        (goto _label Break)))
    (:Completed
      (return (LocalVariables|GetValidTarget)))))