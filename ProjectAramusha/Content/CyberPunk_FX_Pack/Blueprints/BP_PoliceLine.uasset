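; BP_PoliceLine is a cyberpunk FX line panel with text, switchable between a police and an alternate style via IsPolice.
; The construction script sets the style's mesh, solid and wire materials on two overlaid planes, plus text color.
; BeginPlay creates dynamic materials in manual animation mode at zero.
; StartAnim drives both planes' Anim parameter by timeline and, after a short delay, shows the text while a second timeline animates its opacity.
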(event Custom|StartAnim
  (bind _textrender (Variables|Default|GetTextRender))
  (Utilities|FlowControl|Sequence
    (:then_0
      (bind _newtrack_0 (Timeline|Timeline_0 PlayFromStart)
        (:Update
          (Rendering|Material|SetScalarParameterValue (stale EventBeginPlay _returnvalue) "Anim" _newtrack_0 :!class /Script/Engine.MaterialInstanceDynamic)
          (Rendering|Material|SetScalarParameterValue (stale EventBeginPlay _returnvalue_2) "Anim" _newtrack_0 :!class /Script/Engine.MaterialInstanceDynamic))))
    (:then_1
      (Utilities|FlowControl|Delay 0.5)
      (bind _returnvalue (Rendering|Material|CreateDynamicMaterialInstance _textrender 0 (Rendering|Material|GetMaterial _textrender 0) :!class /Script/Engine.PrimitiveComponent))
      (Rendering|Material|SetScalarParameterValue _returnvalue "Opacity" 0.0 :!class /Script/Engine.MaterialInstanceDynamic)
      (Rendering|SetVisibility _textrender true false)
      (bind _newtrack_0_2 (Timeline|Timeline_1 PlayFromStart)
        (:Update
          (Rendering|Material|SetScalarParameterValue _returnvalue "Opacity" _newtrack_0_2 :!class /Script/Engine.MaterialInstanceDynamic))))))

(event EventBeginPlay
  (bind _staticmesh (Variables|Default|GetStaticMesh))
  (bind _sm_plane001_1 (Variables|Default|GetSM_Plane001_1))
  (bind _returnvalue (Rendering|Material|CreateDynamicMaterialInstance _sm_plane001_1 0 (Rendering|Material|GetMaterial _sm_plane001_1 0) :!class /Script/Engine.PrimitiveComponent))
  (Rendering|Material|SetScalarParameterValue _returnvalue "Manual0 Or Auto1?" 0.0 :!class /Script/Engine.MaterialInstanceDynamic)
  (Rendering|Material|SetScalarParameterValue _returnvalue "Anim" 0.0 :!class /Script/Engine.MaterialInstanceDynamic)
  (bind _returnvalue_2 (Rendering|Material|CreateDynamicMaterialInstance _staticmesh 0 (Rendering|Material|GetMaterial _staticmesh 0) :!class /Script/Engine.PrimitiveComponent))
  (Rendering|Material|SetScalarParameterValue _returnvalue_2 "Manual0 Or Auto1?" 0.0 :!class /Script/Engine.MaterialInstanceDynamic)
  (Rendering|Material|SetScalarParameterValue _returnvalue_2 "Anim" 0.0 :!class /Script/Engine.MaterialInstanceDynamic))

(fn ConstructionScript
  (bind _sm_plane001_1 (Variables|Default|GetSM_Plane001_1))
  (bind _staticmesh (Variables|Default|GetStaticMesh))
  (bind _textrender (Variables|Default|GetTextRender))
  (if (Variables|Default|GetIsPolice?)
    (Components|StaticMesh|SetStaticMesh _sm_plane001_1 "/Game/CyberPunk_FX_Pack/Meshes/SM_Plane001_1.SM_Plane001_1")
    (Components|StaticMesh|SetStaticMesh _staticmesh "/Game/CyberPunk_FX_Pack/Meshes/SM_Plane001_1.SM_Plane001_1")
    (Rendering|Material|SetMaterial _sm_plane001_1 0 "/Game/CyberPunk_FX_Pack/Materials/M_PlaneLarge001_1_Inst.M_PlaneLarge001_1_Inst")
    (Rendering|Material|SetMaterial _staticmesh 0 "/Game/CyberPunk_FX_Pack/Materials/M_PlaneLarge001_1Wire.M_PlaneLarge001_1Wire")
    (Rendering|Components|TextRender|SetTextRenderColor _textrender (Math|Color|MakeColor 7 6 1 255))
    (else
      (Components|StaticMesh|SetStaticMesh _sm_plane001_1 "/Game/CyberPunk_FX_Pack/Meshes/SM_PlaneLarge_2.SM_PlaneLarge_2")
      (Components|StaticMesh|SetStaticMesh _staticmesh "/Game/CyberPunk_FX_Pack/Meshes/SM_PlaneLarge_2.SM_PlaneLarge_2")
      (Rendering|Material|SetMaterial _sm_plane001_1 0 "/Game/CyberPunk_FX_Pack/Materials/M_PlaneLarge001_2.M_PlaneLarge001_2")
      (Rendering|Material|SetMaterial _staticmesh 0 "/Game/CyberPunk_FX_Pack/Materials/M_PlaneLarge001_2Wire_Inst.M_PlaneLarge001_2Wire_Inst")
      (Rendering|Components|TextRender|SetTextRenderColor _textrender (Math|Color|MakeColor 255 255 255 255)))))