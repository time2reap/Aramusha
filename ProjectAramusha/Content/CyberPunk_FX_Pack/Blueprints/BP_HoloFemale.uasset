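; BP_HoloFemale is a hologram female effect actor from a cyberpunk FX pack, with Normal and Glitchy looks.
; The construction script uses AnimType to show StaticMesh1 for Normal, or StaticMesh and SMShield1Phase1 for Glitchy.
; BeginPlay is empty, leaving unused a delayed, looping timeline meant to animate the "Anim" parameter on dynamic materials for the two Glitchy meshes.
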(event EventBeginPlay)

(fn ConstructionScript
  (bind _staticmesh (Variables|Default|GetStaticMesh))
  (bind _sm_shield1_phase1 (Variables|Default|GetSM_Shield1_Phase1))
  (bind _staticmesh1 (Variables|Default|GetStaticMesh1))
  (switch Utilities|FlowControl|Switch|SwitchonENUM_HoloFemaleState (Variables|Default|GetAnimType)
    (:NewEnumerator0
      (Rendering|SetVisibility _staticmesh false false)
      (Rendering|SetVisibility _sm_shield1_phase1 false false)
      (Rendering|SetVisibility _staticmesh1 true false))
    (:NewEnumerator1
      (Rendering|SetVisibility _staticmesh true false)
      (Rendering|SetVisibility _sm_shield1_phase1 true false)
      (Rendering|SetVisibility _staticmesh1 false false))))