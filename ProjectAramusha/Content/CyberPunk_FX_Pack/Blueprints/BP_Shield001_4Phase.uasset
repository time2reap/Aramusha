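; Cyberpunk FX shield effect that plays a four-phase animation when StartANIM is called.
; Delays step through the phases, showing one pair of phase components at a time while timelines drive their dynamic materials' "Anim" parameter.
; Phase one also drives the point light's intensity, and during phase three an extra static mesh animates "Anim" and "Opacity".
; The phase four timeline restarts itself on finish, looping the final state.
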(event Custom|StartANIM
  (bind _dynamicmaterials (Variables|Default|GetDynamicMaterials))
  (bind _dynamicmaterials_2 (Variables|Default|GetDynamicMaterials))
  (bind _staticmesh (Variables|Default|GetStaticMesh))
  (bind _dynamicmaterials_3 (Variables|Default|GetDynamicMaterials))
  (bind _dynamicmaterials_4 (Variables|Default|GetDynamicMaterials))
  (for _array_element (Utilities|Array|MakeArray (Variables|Default|GetSM_Shield1_Phase1) (Variables|Default|GetSM_Shield1_Phase2) (Variables|Default|GetSM_Shield1_Phase3) (Variables|Default|GetSM_Shield1_Phase4) (Variables|Default|GetPhase1) (Variables|Default|GetPhase2) (Variables|Default|GetPhase3) (Variables|Default|GetPhase4))
    (bind _returnvalue (Rendering|Material|CreateDynamicMaterialInstance _array_element 0 (Rendering|Material|GetMaterial _array_element 0) :!class /Script/Engine.PrimitiveComponent))
    (Utilities|Array|AddUnique (Variables|Default|GetDynamicMaterials) _returnvalue))
  (Rendering|SetVisibility (Variables|Default|GetSM_Shield1_Phase1) true false)
  (Rendering|SetVisibility (Variables|Default|GetPhase1) true false)
  (for _array_element_2 (Utilities|Array|MakeArray (Variables|Default|GetSM_Shield1_Phase2) (Variables|Default|GetSM_Shield1_Phase3) (Variables|Default|GetSM_Shield1_Phase4) (Variables|Default|GetPhase2) (Variables|Default|GetPhase3) (Variables|Default|GetPhase4))
    (Rendering|SetVisibility _array_element_2 false false))
  (Utilities|FlowControl|Sequence
    (:then_0
      (bind _newtrack_0 (Timeline|Timeline_0 PlayFromStart)
        (:Update
          (Rendering|Material|SetScalarParameterValue (Utilities|Array|Get(acopy) _dynamicmaterials_3) "Anim" _newtrack_0 :!class /Script/Engine.MaterialInstanceDynamic)
          (Rendering|Material|SetScalarParameterValue (Utilities|Array|Get(acopy) _dynamicmaterials_3 4) "Anim" _newtrack_0 :!class /Script/Engine.MaterialInstanceDynamic)
          (Rendering|Components|Light|SetIntensity (Variables|Default|GetPointLight) (* _newtrack_0 3e+04)))))
    (:then_1
      (Utilities|FlowControl|Delay 1.8)
      (Rendering|SetVisibility (Variables|Default|GetSM_Shield1_Phase2) true false)
      (Rendering|SetVisibility (Variables|Default|GetPhase2) true false)
      (for _array_element_3 (Utilities|Array|MakeArray (Variables|Default|GetSM_Shield1_Phase1) (Variables|Default|GetSM_Shield1_Phase3) (Variables|Default|GetSM_Shield1_Phase4) (Variables|Default|GetPhase1) (Variables|Default|GetPhase3) (Variables|Default|GetPhase4))
        (Rendering|SetVisibility _array_element_3 false false))
      (Utilities|FlowControl|Sequence
        (:then_0
          (bind _newtrack_0_2 (Timeline|Timeline_1 PlayFromStart)
            (:Update
              (Rendering|Material|SetScalarParameterValue (Utilities|Array|Get(acopy) _dynamicmaterials_4 1) "Anim" _newtrack_0_2 :!class /Script/Engine.MaterialInstanceDynamic)
              (Rendering|Material|SetScalarParameterValue (Utilities|Array|Get(acopy) _dynamicmaterials_4 5) "Anim" _newtrack_0_2 :!class /Script/Engine.MaterialInstanceDynamic))))
        (:then_1
          (Utilities|FlowControl|Delay 0.8)
          (Rendering|SetVisibility (Variables|Default|GetSM_Shield1_Phase3) true false)
          (Rendering|SetVisibility (Variables|Default|GetPhase3) true false)
          (for _array_element_4 (Utilities|Array|MakeArray (Variables|Default|GetSM_Shield1_Phase1) (Variables|Default|GetSM_Shield1_Phase2) (Variables|Default|GetSM_Shield1_Phase4) (Variables|Default|GetPhase1) (Variables|Default|GetPhase2) (Variables|Default|GetPhase4))
            (Rendering|SetVisibility _array_element_4 false false))
          (Utilities|FlowControl|Sequence
            (:then_0
              (bind _newtrack_0_3 (Timeline|Timeline_2 PlayFromStart)
                (:Update
                  (Rendering|Material|SetScalarParameterValue (Utilities|Array|Get(acopy) _dynamicmaterials 2) "Anim" _newtrack_0_3 :!class /Script/Engine.MaterialInstanceDynamic)
                  (Rendering|Material|SetScalarParameterValue (Utilities|Array|Get(acopy) _dynamicmaterials 6) "Anim" _newtrack_0_3 :!class /Script/Engine.MaterialInstanceDynamic))))
            (:then_1
              (Utilities|FlowControl|Delay 0.5)
              (bind _returnvalue_2 (Rendering|Material|CreateDynamicMaterialInstance _staticmesh 0 (Rendering|Material|GetMaterial _staticmesh 0) :!class /Script/Engine.PrimitiveComponent))
              (Utilities|FlowControl|Sequence
                (:then_0
                  (bind _newtrack_0_4 (Timeline|Timeline_4 PlayFromStart)
                    (:Update
                      (Rendering|Material|SetScalarParameterValue _returnvalue_2 "Anim" _newtrack_0_4 :!class /Script/Engine.MaterialInstanceDynamic))))
                (:then_1
                  (bind _newtrack_0_5 (Timeline|Timeline_5 PlayFromStart)
                    (:Update
                      (Rendering|Material|SetScalarParameterValue _returnvalue_2 "Opacity" _newtrack_0_5 :!class /Script/Engine.MaterialInstanceDynamic))))))
            (:then_2
              (Utilities|FlowControl|Delay 1.2)
              (Rendering|SetVisibility (Variables|Default|GetSM_Shield1_Phase4) true false)
              (Rendering|SetVisibility (Variables|Default|GetPhase4) true false)
              (for _array_element_5 (Utilities|Array|MakeArray (Variables|Default|GetSM_Shield1_Phase1) (Variables|Default|GetSM_Shield1_Phase2) (Variables|Default|GetSM_Shield1_Phase3) (Variables|Default|GetPhase1) (Variables|Default|GetPhase2) (Variables|Default|GetPhase3))
                (Rendering|SetVisibility _array_element_5 false false))
              (bind _newtrack_0_6 (Timeline|Timeline_3 PlayFromStart)
                (:Update
                  (Rendering|Material|SetScalarParameterValue (Utilities|Array|Get(acopy) _dynamicmaterials_2 3) "Anim" _newtrack_0_6 :!class /Script/Engine.MaterialInstanceDynamic)
                  (Rendering|Material|SetScalarParameterValue (Utilities|Array|Get(acopy) _dynamicmaterials_2 7) "Anim" _newtrack_0_6 :!class /Script/Engine.MaterialInstanceDynamic))
                (:Finished
                  (Utilities|FlowControl|Sequence
                    (:then_0
                      (Timeline|Timeline_3 PlayFromStart))))))))))))

(fn ConstructionScript)