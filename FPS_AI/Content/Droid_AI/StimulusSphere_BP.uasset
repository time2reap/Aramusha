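; Short-lived stimulus actor that alerts nearby droid AI and points them toward a disturbance.
; On BeginPlay it sets a half-second lifespan and scans DetectionSphere for living, unalerted droids, writing Alerted and a RotateTarget facing itself to their blackboards.
; Droids that begin overlapping get the same alert, but facing AlertLoc, and only if their controller has not started combat.
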(event OnComponentBeginOverlap(DetectionSphere)
  (params (OverlappedComponent :type Primitive%20Component%20Object%20Reference) (OtherActor :type Actor%20Object%20Reference) (OtherComp :type Primitive%20Component%20Object%20Reference) (OtherBodyIndex :type Integer) (bFromSweep :type Boolean) (SweepResult :type Hit%20Result%20Structure%20%28by%20ref%29))
  (bind _asdroid_ai_blueprint (Utilities|Casting|CastToDroidAI_Blueprint OtherActor))
  (if (not (Variables|/Game/Droid_AI/DroidAI_Controller.DroidAI_Controller_C|GetCombatStarted (Variables|/Game/Droid_AI/DroidAI_Blueprint.DroidAI_Blueprint_C|GetEnemyAI_Controller _asdroid_ai_blueprint)))
    (if (and (Variables|/Game/Droid_AI/DroidAI_Blueprint.DroidAI_Blueprint_C|GetAlive _asdroid_ai_blueprint) (not (ScalableFloat|GetValueasBool (AI|GetBlackboard _asdroid_ai_blueprint) (Utilities|Name|MakeLiteralName "Alerted"))))
      (Class|BlackboardComponent|SetValueasRotator (AI|GetBlackboard _asdroid_ai_blueprint) (Utilities|Name|MakeLiteralName "RotateTarget") (Math|Rotator|FindLookatRotation (Transformation|GetActorLocation _asdroid_ai_blueprint) (Variables|Default|GetAlertLoc)))
      (AI|Components|Blackboard|SetValueasBool (AI|GetBlackboard _asdroid_ai_blueprint) (Utilities|Name|MakeLiteralName "Alerted") true))))

(event EventBeginPlay
  (Actor|SetLifeSpan 0.5)
  (for _array_element (Collision|GetOverlappingActors (Variables|Default|GetDetectionSphere) "/Game/Droid_AI/DroidAI_Blueprint.DroidAI_Blueprint_C" :!class /Script/Engine.PrimitiveComponent)
    (bind _asdroid_ai_blueprint (Utilities|Casting|CastToDroidAI_Blueprint _array_element))
    (if (and (Variables|/Game/Droid_AI/DroidAI_Blueprint.DroidAI_Blueprint_C|GetAlive _asdroid_ai_blueprint) (not (ScalableFloat|GetValueasBool (AI|GetBlackboard _asdroid_ai_blueprint) (Utilities|Name|MakeLiteralName "Alerted"))))
      (Class|BlackboardComponent|SetValueasRotator (AI|GetBlackboard _asdroid_ai_blueprint) (Utilities|Name|MakeLiteralName "RotateTarget") (Math|Rotator|FindLookatRotation (Transformation|GetActorLocation _asdroid_ai_blueprint) (Transformation|GetActorLocation)))
      (AI|Components|Blackboard|SetValueasBool (AI|GetBlackboard _asdroid_ai_blueprint) (Utilities|Name|MakeLiteralName "Alerted") true))))

(fn ConstructionScript)