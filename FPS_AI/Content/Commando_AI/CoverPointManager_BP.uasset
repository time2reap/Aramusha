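; Cover point manager for Commando AI that tracks level cover points and spawns commandos above randomly picked unoccupied ones.
; It gathers all cover points and the player at BeginPlay, with events to return or remove points from the pool.
; Search functions rank points by distance to AI or player, using line traces to require cover from the player and an angle check when retreating.
; Chosen points are marked occupied and usually removed, except by random search.
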(event Custom|SpawnNewBaddies
  (params (NumBaddies :type Integer))
  (bind _currentcoverpoints (Variables|Default|GetCurrentCoverPoints))
  (for _index (range 0 NumBaddies)
    (bind _output_get (Variables|Default|SetcurrNode (Utilities|Array|Get(acopy) _currentcoverpoints (Math|Random|RandomIntegerinRange 0 (- (Utilities|Array|Length _currentcoverpoints) 1)))))
    (Utilities|IsValid _output_get
      (:Is%20Valid
        (if (not (Variables|/Game/Commando_AI/CoverPoint_Blueprint.CoverPoint_Blueprint_C|GetOccupied _output_get))
          (Variables|/Game/Commando_AI/CoverPoint_Blueprint.CoverPoint_Blueprint_C|SetOccupied _output_get true)
          (AI|SpawnAIFromClass "/Game/Commando_AI/CommandoAI_Blueprint.CommandoAI_Blueprint_C" 0 (+ (Transformation|GetActorLocation (Variables|Default|GetcurrNode)) (* (Transformation|GetActorUpVector (Variables|Default|GetcurrNode)) 1e+03)) "0, 0, 0" true))))))

(event Custom|RemoveCoverPoint
  (params (PointToRemove :type Cover%20Point%20Blueprint%20Object%20Reference))
  (Utilities|IsValid PointToRemove
    (:Is%20Valid
      (Utilities|Array|RemoveItem (Variables|Default|GetCurrentCoverPoints) PointToRemove)
      (Variables|/Game/Commando_AI/CoverPoint_Blueprint.CoverPoint_Blueprint_C|SetOccupied PointToRemove true))))

(event Custom|AddCoverPoint
  (params (NewCoverPoint :type Cover%20Point%20Blueprint%20Object%20Reference))
  (Utilities|IsValid NewCoverPoint
    (:Is%20Valid
      (Utilities|Array|AddUnique (Variables|Default|GetCurrentCoverPoints) NewCoverPoint)
      (Variables|/Game/Commando_AI/CoverPoint_Blueprint.CoverPoint_Blueprint_C|SetOccupied NewCoverPoint false))))

(event EventBeginPlay
  (bind _outactors (Actor|GetAllActorsOfClass "/Game/Commando_AI/CoverPoint_Blueprint.CoverPoint_Blueprint_C"))
  (Variables|Default|SetCurrentCoverPoints _outactors)
  (bind _outactors_2 (Actor|GetAllActorsOfClass "/Game/FirstPersonBP/Blueprints/FirstPersonCharacter.FirstPersonCharacter_C"))
  (Variables|Default|SetPlayer (Utilities|Array|Get(acopy) _outactors_2)))

(fn ConstructionScript)

(fn FindAcceptableCover
  (params (AI%20Pawn :type Actor%20Object%20Reference) (AcceptableRadius :type Float%20%28single-precision%29) (DesiredRadius :type Float%20%28single-precision%29))
  (for _array_element (Variables|Default|GetCurrentCoverPoints)
    (bind _validcover (CallFunction|CovertoObjectRaycast _array_element (Variables|Default|GetPlayer)))
    (if _validcover
      ;[1 1 1] If the distance is less than our auto accept distance
      (if (< (Transformation|GetHorizontalDistanceTo AI%20Pawn _array_element) DesiredRadius)
        (Variables|/Game/Commando_AI/CoverPoint_Blueprint.CoverPoint_Blueprint_C|SetOccupied _array_element true)
        (return true _array_element)
        (else
          ;[1 1 1] Otherwise, ensure its in an acceptable range and proceed to find the closest one
          (if (< (Transformation|GetHorizontalDistanceTo AI%20Pawn _array_element) AcceptableRadius)
            (if (< (Transformation|GetHorizontalDistanceTo AI%20Pawn _array_element) (LocalVariables|GetBestDist))
              (LocalVariables|SetBestDist (Transformation|GetHorizontalDistanceTo AI%20Pawn _array_element))
              (LocalVariables|SetReturnPoint _array_element)))))))
  ;[1 1 1] If we looped through all of the cover points, then we return a point if we found one
  (Utilities|IsValid (LocalVariables|GetReturnPoint)
    (:Is%20Valid
      (Variables|/Game/Commando_AI/CoverPoint_Blueprint.CoverPoint_Blueprint_C|SetOccupied (LocalVariables|GetReturnPoint) true)
      (CallFunction|RemoveCoverPoint (LocalVariables|GetReturnPoint))
      (return true (LocalVariables|GetReturnPoint)))
    (:Is%20Not%20Valid
      (return false 0))))

(fn FindBestCover
  (params (AI%20Pawn :type Actor%20Object%20Reference) (AcceptableRadius :type Float%20%28single-precision%29) (FavorClose :type Boolean) (AutoAcceptRadius :type Float%20%28single-precision%29))
  (if FavorClose
    (LocalVariables|SetBestNodeValue 1e+08)
    (else
      (LocalVariables|SetBestNodeValue 0.0)))
  ;[1 1 1] Gather Node information
  (for _array_element (Variables|Default|GetCurrentCoverPoints)
    (bind _validcover (CallFunction|CovertoObjectRaycast _array_element (Variables|Default|GetPlayer)))
    (if _validcover
      (LocalVariables|SetCurrDist (Transformation|GetHorizontalDistanceTo AI%20Pawn _array_element))
      (LocalVariables|SetDistFromPlayer (Transformation|GetHorizontalDistanceTo _array_element (Variables|Default|GetPlayer)))
      (if FavorClose
        ;[1 1 1] Ensure its in an acceptable range and proceed to find the closest one
        (if (< (LocalVariables|GetCurrDist) AutoAcceptRadius)
          (LocalVariables|SetReturnPoint _array_element)
          ;[1 1 1] If we looped through all of the cover points, then we return a point if we found one
          (Utilities|IsValid (LocalVariables|GetReturnPoint)
            (:Is%20Valid
              (Variables|/Game/Commando_AI/CoverPoint_Blueprint.CoverPoint_Blueprint_C|SetOccupied (LocalVariables|GetReturnPoint) true)
              (CallFunction|RemoveCoverPoint (LocalVariables|GetReturnPoint))
              (return true (LocalVariables|GetReturnPoint)))
            (:Is%20Not%20Valid
              (return false 0)))
          (else
            (bind _ascommando_ai_controller (Utilities|Casting|CastToCommandoAI_Controller (AI|GetAIController AI%20Pawn)))
            (if (Math|Boolean|ANDBoolean (< (LocalVariables|GetCurrDist) AcceptableRadius) (> (LocalVariables|GetDistFromPlayer) (Variables|/Game/Commando_AI/CommandoAI_Controller.CommandoAI_Controller_C|GetTooCloseDist _ascommando_ai_controller)) (< (* (Math|Float|MakeLiteralFloat 1.0) (LocalVariables|GetCurrDist)) (LocalVariables|GetBestNodeValue)))
              (LocalVariables|SetBestNodeValue (* (Math|Float|MakeLiteralFloat 1.0) (LocalVariables|GetCurrDist)))
              (LocalVariables|SetReturnPoint _array_element))))
        (else
          ;[1 1 1] Ensure its in an acceptable range and proceed to find a distant one
          (if (and (< (LocalVariables|GetCurrDist) AcceptableRadius) (> (* (Math|Float|MakeLiteralFloat 1.0) (LocalVariables|GetCurrDist)) (LocalVariables|GetBestNodeValue)))
            (LocalVariables|SetBestNodeValue (* (Math|Float|MakeLiteralFloat 1.0) (LocalVariables|GetCurrDist)))
            (LocalVariables|SetReturnPoint _array_element))))))
  (Utilities|IsValid (LocalVariables|GetReturnPoint)
    (:Is%20Valid
      (Variables|/Game/Commando_AI/CoverPoint_Blueprint.CoverPoint_Blueprint_C|SetOccupied (LocalVariables|GetReturnPoint) true)
      (CallFunction|RemoveCoverPoint (LocalVariables|GetReturnPoint))
      (return true (LocalVariables|GetReturnPoint)))
    (:Is%20Not%20Valid
      (return false 0))))

(fn CovertoObjectRaycast
  (params (CoverPoint :type Cover%20Point%20Blueprint%20Object%20Reference) (Object :type Actor%20Object%20Reference))
  (bind (_outhit _returnvalue) (Collision|LineTraceByChannel (+ (* (Math|Vector|GetUpVector (Variables|/Script/Engine.Actor|GetRootComponent CoverPoint)) 1e+02) (Transformation|GetActorLocation CoverPoint)) (Transformation|GetActorLocation Object) "TraceTypeQuery1" false 0 "None" true "(R=1.000000,G=0.959540,B=0.000000,A=1.000000)" "(R=0.000000,G=1.000000,B=0.000000,A=1.000000)" 3.0))
  (if _returnvalue
    (if (== (.HitActor (Collision|BreakHitResult _outhit)) (Variables|Default|GetPlayer))
      (return false)
      (else
        _)))
  (return true))

(fn FindCoverBasedonPlayer
  (params (AI%20Pawn :type Actor%20Object%20Reference) (AcceptableRadius :type Float%20%28single-precision%29) (FavorClose :type Boolean) (Retreating? :type Boolean))
  (bind _player (Variables|Default|GetPlayer))
  (if FavorClose
    (LocalVariables|SetBestNodeValue 1e+08)
    (LocalVariables|SetCurrentCoverDist (Transformation|GetHorizontalDistanceTo AI%20Pawn (Variables|Default|GetPlayer)))
    (else
      (LocalVariables|SetBestNodeValue 0.0)))
  (for _array_element (Variables|Default|GetCurrentCoverPoints)
    (if FavorClose
      ;[1 1 1] Ensure its in an acceptable range and proceed to find the closest one
      (bind _output_get (LocalVariables|SetCurrentDist (Transformation|GetHorizontalDistanceTo _array_element (Variables|Default|GetPlayer))))
      (if Retreating?
        (bind _isbehind (CallFunction|CheckIsBehindEnemy _array_element AI%20Pawn))
        (if _isbehind
          (bind _validcover (CallFunction|CovertoObjectRaycast _array_element (Variables|Default|GetPlayer) :!label _label))
          (if _validcover
            (bind _ascommando_ai_controller (Utilities|Casting|CastToCommandoAI_Controller (AI|GetAIController AI%20Pawn)))
            (if (Math|Boolean|ANDBoolean (< (Transformation|GetHorizontalDistanceTo AI%20Pawn _array_element) AcceptableRadius) (< _output_get (LocalVariables|GetCurrentCoverDist)) (> (LocalVariables|GetCurrentDist) (+ (Variables|/Game/Commando_AI/CommandoAI_Controller.CommandoAI_Controller_C|GetTooCloseDist _ascommando_ai_controller) 5e+01)) (< (Transformation|GetHorizontalDistanceTo AI%20Pawn _array_element) (LocalVariables|GetBestNodeValue)))
              (LocalVariables|SetBestNodeValue (Transformation|GetHorizontalDistanceTo AI%20Pawn _array_element))
              (LocalVariables|SetReturnPoint _array_element))))
        (else
          (goto _label)))
      (else
        ;[1 1 1] Ensure its in an acceptable range and proceed to find a distant one
        (bind _output_get_2 (LocalVariables|SetCurrentDist (Transformation|GetHorizontalDistanceTo _array_element _player)))
        (if (Math|Boolean|ANDBoolean (< _output_get_2 AcceptableRadius) (> _output_get_2 (Transformation|GetHorizontalDistanceTo AI%20Pawn _player)) (> (LocalVariables|GetCurrentDist) (LocalVariables|GetBestNodeValue)))
          (bind _validcover_2 (CallFunction|CovertoObjectRaycast _array_element (Variables|Default|GetPlayer)))
          (if _validcover_2
            (LocalVariables|SetBestNodeValue (LocalVariables|GetCurrentDist))
            (LocalVariables|SetReturnPoint _array_element))))))
  ;[1 1 1] If we looped through all of the cover points, then we return a point if we found one
  (Utilities|IsValid (LocalVariables|GetReturnPoint)
    (:Is%20Valid
      (Variables|/Game/Commando_AI/CoverPoint_Blueprint.CoverPoint_Blueprint_C|SetOccupied (LocalVariables|GetReturnPoint) true)
      (CallFunction|RemoveCoverPoint (LocalVariables|GetReturnPoint))
      (return true (LocalVariables|GetReturnPoint)))
    (:Is%20Not%20Valid
      (return false 0))))

(fn GetAngleBetweenVectors
  (params (V1 :type Vector) (V2 :type Vector))
  (return (Class|KismetMathLibrary|DegAcos (Math|Vector|DotProduct (Math|Vector|Normalize V1) (Math|Vector|Normalize V2)))))

(fn CheckIsBehindEnemy
  (params (CoverPoint :type Cover%20Point%20Blueprint%20Object%20Reference) (EnemyPawn :type Actor%20Object%20Reference))
  (bind _angle (CallFunction|GetAngleBetweenVectors (Math|Vector|Normalize (- (Transformation|GetActorLocation EnemyPawn) (Transformation|GetActorLocation CoverPoint))) (Transformation|GetActorForwardVector EnemyPawn)))
  (return (< _angle 9e+01)))

(fn FindRandomCover
  (params (AI%20Pawn :type Pawn%20Object%20Reference))
  (bind _currentcoverpoints (Variables|Default|GetCurrentCoverPoints))
  (Variables|Default|SetcurrNode 0)
  (for _array_element _currentcoverpoints
    (bind _output_get (Variables|Default|SetcurrNode (Utilities|Array|Get(acopy) _currentcoverpoints (Math|Random|RandomIntegerinRange 0 (- (Utilities|Array|Length _currentcoverpoints) 1)))))
    (if (and (Variables|/Game/Commando_AI/CoverPoint_Blueprint.CoverPoint_Blueprint_C|GetOccupied _output_get) (> (Transformation|GetHorizontalDistanceTo _output_get AI%20Pawn) 3e+02))
      (return true (Variables|Default|GetcurrNode))))
  (return (Utilities|IsValid (Variables|Default|GetcurrNode)) (Variables|Default|GetcurrNode)))