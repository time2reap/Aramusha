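; Goal point for the commando AI squad that stages the gunship finale and ends the game.
; On BeginPlay and CommanderDied it gathers living commandos, making the first the commander with this actor as blackboard goal.
; A commando entering the box, once GunshipReady, sends the squad to post-up points on a finishing behavior tree.
; The hidden gunship then appears, moves through two timeline-driven interpolated legs with delayed smoke, and the game quits.
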(event OnComponentBeginOverlap(Box)
  (params (OverlappedComponent :type Primitive%20Component%20Object%20Reference) (OtherActor :type Actor%20Object%20Reference) (OtherComp :type Primitive%20Component%20Object%20Reference) (OtherBodyIndex :type Integer) (bFromSweep :type Boolean) (SweepResult :type Hit%20Result%20Structure%20%28by%20ref%29))
  (bind _gunship (Variables|Default|GetGunship))
  (bind _gunship_2 (Variables|Default|GetGunship))
  (Utilities|Casting|CastToCommandoAI_Blueprint OtherActor)
  (if (Variables|Default|GetGunshipReady)
    (Variables|Default|SetGunshipReady false)
    (bind _outactors (Actor|GetAllActorsOfClass "/Game/Commando_AI/CommandoAI_Blueprint.CommandoAI_Blueprint_C"))
    (Variables|Default|SetCommandos _outactors)
    (for (_array_element _array_index) (Variables|Default|GetPostUpPoints)
      (if (and (Utilities|Array|IsValidIndex (Variables|Default|GetCommandos) _array_index) (Variables|/Game/Commando_AI/CommandoAI_Blueprint.CommandoAI_Blueprint_C|GetAlive (Utilities|Array|Get(acopy) (Variables|Default|GetCommandos) _array_index)))
        (AI|RunBehaviorTree (AI|GetAIController (Utilities|Array|Get(acopy) (Variables|Default|GetCommandos) _array_index)) "/Game/Commando_AI/Commando_Finished_BHT.Commando_Finished_BHT")
        (AI|Components|Blackboard|SetValueasBool (AI|GetBlackboard (AI|GetAIController (Utilities|Array|Get(acopy) (Variables|Default|GetCommandos) _array_index))) (Utilities|Name|MakeLiteralName "PostingUp") true)
        (AI|Components|Blackboard|SetValueasObject (AI|GetBlackboard (AI|GetAIController (Utilities|Array|Get(acopy) (Variables|Default|GetCommandos) _array_index))) (Utilities|Name|MakeLiteralName "PostUpPoint") _array_element)
        (Class|BlackboardComponent|SetValueasRotator (AI|GetBlackboard (AI|GetAIController (Utilities|Array|Get(acopy) (Variables|Default|GetCommandos) _array_index))) (Utilities|Name|MakeLiteralName "RotateTarget") (Transformation|GetActorRotation _array_element))))
    (Utilities|FlowControl|Delay 2.0)
    (CallFunction|ActivateSmoke)
    (Rendering|SetVisibility (Variables|/Game/Misc/Gunship_BP.Gunship_BP_C|GetShip _gunship_2) true false)
    (bind _alpha (Timeline|Gunship_TL PlayFromStart)
      (:Update
        (Transformation|SetActorLocation _gunship_2 (Math|Interpolation|VInterpTo (Transformation|GetActorLocation _gunship_2) (Variables|/Game/Misc/Gunship_BP.Gunship_BP_C|GetEndLoc _gunship_2) _alpha 0.01) false false)
        (Transformation|SetActorRotation _gunship_2 (Math|Interpolation|RInterpTo (Transformation|GetActorRotation _gunship_2) (Variables|/Game/Misc/Gunship_BP.Gunship_BP_C|GetEndRot _gunship_2) _alpha 0.005)))
      (:Finished
        (Utilities|FlowControl|Delay 2.0)
        (bind _alpha_2 (Timeline|Timeline_0 PlayFromStart)
          (:Update
            (Transformation|SetActorLocation _gunship (Math|Interpolation|VInterpTo (Transformation|GetActorLocation _gunship) (Variables|/Game/Misc/Gunship_BP.Gunship_BP_C|GetEndLoc2 _gunship) _alpha_2 0.015) false false)
            (Transformation|SetActorRotation _gunship (Math|Interpolation|RInterpTo (Transformation|GetActorRotation _gunship) (Variables|/Game/Misc/Gunship_BP.Gunship_BP_C|GetEndRot2 _gunship) _alpha_2 0.02)))
          (:Finished
            (Game|QuitGame 0 "Quit")))))))

(event Custom|CommanderDied
  (Utilities|Array|Clear (Variables|Default|GetCommandos))
  (bind _outactors (Actor|GetAllActorsOfClass "/Game/Commando_AI/CommandoAI_Blueprint.CommandoAI_Blueprint_C"))
  (for _array_element _outactors
    (Utilities|IsValid _array_element
      (:Is%20Valid
        (if (Variables|/Game/Commando_AI/CommandoAI_Blueprint.CommandoAI_Blueprint_C|GetAlive _array_element)
          (Utilities|Array|Add (Variables|Default|GetCommandos) _array_element)))))
  (for (_array_element_2 _array_index) (Variables|Default|GetCommandos)
    (Default|SetCommanderStatus _array_element_2 (== 0 _array_index))
    (Variables|/Game/Commando_AI/CommandoAI_Controller.CommandoAI_Controller_C|SetCommandoIndex (Variables|/Game/Commando_AI/CommandoAI_Blueprint.CommandoAI_Blueprint_C|GetEnemyAI_Controller _array_element_2) _array_index)
    (if (== 0 _array_index)
      (bind _output_get (Variables|Default|SetCurrentCommander _array_element_2))
      (AI|Components|Blackboard|SetValueasObject (AI|GetBlackboard (AI|GetAIController _output_get)) (Utilities|Name|MakeLiteralName "GoalPoint") self)
      (AI|Components|Blackboard|SetValueasObject (AI|GetBlackboard (AI|GetAIController _output_get)) (Utilities|Name|MakeLiteralName "SquadLeader") _output_get)))
  (Rendering|SetVisibility (Variables|/Game/Misc/Gunship_BP.Gunship_BP_C|GetShip (Variables|Default|GetGunship)) false false))

(event Custom|ActivateSmoke
  (Utilities|FlowControl|Delay 6.0)
  (Components|Activation|Activate (Variables|/Game/Misc/Gunship_BP.Gunship_BP_C|GetParticleSystem (Variables|Default|GetGunship)) true))

(event EventBeginPlay
  (bind _outactors (Actor|GetAllActorsOfClass "/Game/Commando_AI/CommandoAI_Blueprint.CommandoAI_Blueprint_C"))
  (for _array_element _outactors
    (Utilities|IsValid _array_element
      (:Is%20Valid
        (if (Variables|/Game/Commando_AI/CommandoAI_Blueprint.CommandoAI_Blueprint_C|GetAlive _array_element)
          (Utilities|Array|Add (Variables|Default|GetCommandos) _array_element)))))
  (for (_array_element_2 _array_index) (Variables|Default|GetCommandos)
    (Default|SetCommanderStatus _array_element_2 (== 0 _array_index))
    (Variables|/Game/Commando_AI/CommandoAI_Controller.CommandoAI_Controller_C|SetCommandoIndex (Variables|/Game/Commando_AI/CommandoAI_Blueprint.CommandoAI_Blueprint_C|GetEnemyAI_Controller _array_element_2) _array_index)
    (if (== 0 _array_index)
      (bind _output_get (Variables|Default|SetCurrentCommander _array_element_2))
      (AI|Components|Blackboard|SetValueasObject (AI|GetBlackboard (AI|GetAIController _output_get)) (Utilities|Name|MakeLiteralName "GoalPoint") self)
      (AI|Components|Blackboard|SetValueasObject (AI|GetBlackboard (AI|GetAIController _output_get)) (Utilities|Name|MakeLiteralName "SquadLeader") _output_get)))
  (Rendering|SetVisibility (Variables|/Game/Misc/Gunship_BP.Gunship_BP_C|GetShip (Variables|Default|GetGunship)) false false))

(fn ConstructionScript)