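; Trigger actor that sends a commando AI squad to post up at preset TargetPoints when the commander first overlaps it.
; If the commander is not in combat, it gathers every commando in the level, commander first, and pairs them to points by array index.
; It writes each one's location, rotation and post-up/cover blackboard keys and sets walk speed.
; It destroys itself afterwards, or immediately if the commander is in combat.
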(event Collision|EventActorBeginOverlap
  (params (OtherActor :type Actor%20Object%20Reference))
  (bind _commandos (Variables|Default|GetCommandos))
  (bind _commandos_2 (Variables|Default|GetCommandos))
  (if (not (Variables|Default|GetActivated))
    (bind _ascommando_ai_blueprint (Utilities|Casting|CastToCommandoAI_Blueprint OtherActor))
    (if (Variables|/Game/Commando_AI/CommandoAI_Controller.CommandoAI_Controller_C|GetIsCommander? (Variables|/Game/Commando_AI/CommandoAI_Blueprint.CommandoAI_Blueprint_C|GetEnemyAI_Controller _ascommando_ai_blueprint))
      (Variables|Default|SetActivated true)
      (if (ScalableFloat|GetValueasBool (AI|GetBlackboard _ascommando_ai_blueprint) (Utilities|Name|MakeLiteralName "InCombat"))
        (Actor|DestroyActor)
        (else
          (Utilities|Array|Add _commandos _ascommando_ai_blueprint)
          (bind _outactors (Actor|GetAllActorsOfClass "/Game/Commando_AI/CommandoAI_Blueprint.CommandoAI_Blueprint_C"))
          (for _array_element _outactors
            (Utilities|Array|AddUnique _commandos _array_element))
          (for (_array_element_2 _array_index) (Variables|Default|GetTargetPoints)
            (if (Utilities|Array|IsValidIndex _commandos_2 _array_index)
              (Class|BlackboardComponent|SetValueasRotator (AI|GetBlackboard (Utilities|Array|Get(acopy) _commandos_2 _array_index)) (Utilities|Name|MakeLiteralName "RotateTarget") (Transformation|GetActorRotation _array_element_2))
              (AI|Components|Blackboard|SetValueasVector (AI|GetBlackboard (Utilities|Array|Get(acopy) _commandos_2 _array_index)) (Utilities|Name|MakeLiteralName "MoveToPoint") (Transformation|GetActorLocation _array_element_2))
              (AI|Components|Blackboard|SetValueasBool (AI|GetBlackboard (Utilities|Array|Get(acopy) _commandos_2 _array_index)) (Utilities|Name|MakeLiteralName "PostingUp") true)
              (AI|Components|Blackboard|SetValueasObject (AI|GetBlackboard (Utilities|Array|Get(acopy) _commandos_2 _array_index)) (Utilities|Name|MakeLiteralName "PostUpPoint") _array_element_2)
              (AI|Components|Blackboard|SetValueasBool (AI|GetBlackboard (Utilities|Array|Get(acopy) _commandos_2 _array_index)) (Utilities|Name|MakeLiteralName "InCover") true)
              (Variables|/Script/Engine.CharacterMovementComponent|SetMaxWalkSpeed (Variables|/Script/Engine.Character|GetCharacterMovement (Utilities|Array|Get(acopy) _commandos_2 _array_index)) 3e+02)))
          (Actor|DestroyActor))))))

(fn ConstructionScript)